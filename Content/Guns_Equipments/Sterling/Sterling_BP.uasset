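; Sterling weapon Blueprint that fires projectiles, manages clip and reserve ammo, and drives camera recoil.
; Each shot spawns a projectile at the muzzle, spends ammo and sphere-traces forward, calling Threathed on an Enemy hit.
; A timeline adds pitch and yaw while firing.
; On stop it reverses faster, scaling recovery by the pitch difference between rotations captured at recoil start and release, against a threshold.
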(event Custom|Fire
  (if (not (<= (Variables|Default|GetAmmo) 0))
    (Game|SpawnActorfromClass "/Game/Guns_Equipments/Ak47/Projectile.Projectile_C" (Transformation|GetWorldTransform (Variables|Default|GetMuzzle)) "Undefined" "OverrideRootScale" 0 0)
    (CallFunction|ThreatTrace (Variables|Default|GetThreatLevel))
    (Variables|Default|SetAmmo (- (Variables|Default|GetAmmo) 1))))

(event Custom|CE_OnFire
  (Components|Activation|Activate (Variables|Default|GetNiagara) false)
  (CallFunction|Fire)
  (Components|Timeline|SetPlayRate (Variables|Default|GetRecoilTimeline) 1.0)
  (Utilities|FlowControl|Sequence
    (:then_0
      (Utilities|FlowControl|DoOnce false
        (:Completed
          (Variables|Default|SetOriginRotation (Pawn|GetControlRotation (Game|GetPlayerController 0) :!class /Script/Engine.Controller)))))
    (:then_1
      (bind (_direction _pitchinput _yawinput) (Timeline|RecoilTimeline Play)
        (:Update
          (switch Utilities|FlowControl|Switch|SwitchonETimelineDirection _direction
            (:Forward
              (CallFunction|UpdatePlayerPitchandYaw _pitchinput _yawinput))
            (:Backward
              (Utilities|FlowControl|Sequence
                (:then_0
                  (Utilities|FlowControl|DoOnce false
                    (:Completed
                      (Variables|Default|SetPostRotation (Pawn|GetControlRotation (Game|GetPlayerController 0) :!class /Script/Engine.Controller)))))
                (:then_1
                  (CallFunction|UpdatePlayerPitchandYaw (* _pitchinput -13.0 (select (> (Math|Float|Absolute(Float) (.Pitch (Math|Rotator|BreakRotator (Math|Rotator|Delta(Rotator) (Variables|Default|GetOriginRotation) (Variables|Default|GetPostRotation))))) (Variables|Default|GetRecoilMaxThreshold)) (Math|Float|MapRangeClamped (Math|Float|Absolute(Float) (.Pitch (Math|Rotator|BreakRotator (Math|Rotator|Delta(Rotator) (Variables|Default|GetOriginRotation) (Variables|Default|GetPostRotation))))) (Variables|Default|GetRecoilMaxThreshold) 3e+01 1.0 0.0) (Math|Float|MapRangeClamped (Math|Float|Absolute(Float) (.Pitch (Math|Rotator|BreakRotator (Math|Rotator|Delta(Rotator) (Variables|Default|GetOriginRotation) (Variables|Default|GetPostRotation))))) 0.0 (Variables|Default|GetRecoilMaxThreshold) 0.0 1.0))) (* _yawinput -3.0 (select (> (Math|Float|Absolute(Float) (.Pitch (Math|Rotator|BreakRotator (Math|Rotator|Delta(Rotator) (Variables|Default|GetOriginRotation) (Variables|Default|GetPostRotation))))) (Variables|Default|GetRecoilMaxThreshold)) (Math|Float|MapRangeClamped (Math|Float|Absolute(Float) (.Pitch (Math|Rotator|BreakRotator (Math|Rotator|Delta(Rotator) (Variables|Default|GetOriginRotation) (Variables|Default|GetPostRotation))))) (Variables|Default|GetRecoilMaxThreshold) 3e+01 1.0 0.0) (Math|Float|MapRangeClamped (Math|Float|Absolute(Float) (.Pitch (Math|Rotator|BreakRotator (Math|Rotator|Delta(Rotator) (Variables|Default|GetOriginRotation) (Variables|Default|GetPostRotation))))) 0.0 (Variables|Default|GetRecoilMaxThreshold) 0.0 1.0)))))))))
        (:Finished
          (switch Utilities|FlowControl|Switch|SwitchonETimelineDirection _direction
            (:Backward
              (CallFunction|ResetRecoil))))))))

(event Custom|CE_StopFire
  (Components|Activation|Deactivate (Variables|Default|GetNiagara))
  (Components|Timeline|SetPlayRate (Variables|Default|GetRecoilTimeline) 13.0)
  (bind (_direction _pitchinput _yawinput) (Timeline|RecoilTimeline Reverse)
    (:Update
      (switch Utilities|FlowControl|Switch|SwitchonETimelineDirection _direction
        (:Forward
          (CallFunction|UpdatePlayerPitchandYaw _pitchinput _yawinput))
        (:Backward
          (Utilities|FlowControl|Sequence
            (:then_0
              (Utilities|FlowControl|DoOnce false
                (:Completed
                  (Variables|Default|SetPostRotation (Pawn|GetControlRotation (Game|GetPlayerController 0) :!class /Script/Engine.Controller)))))
            (:then_1
              (CallFunction|UpdatePlayerPitchandYaw (* _pitchinput -13.0 (select (> (Math|Float|Absolute(Float) (.Pitch (Math|Rotator|BreakRotator (Math|Rotator|Delta(Rotator) (Variables|Default|GetOriginRotation) (Variables|Default|GetPostRotation))))) (Variables|Default|GetRecoilMaxThreshold)) (Math|Float|MapRangeClamped (Math|Float|Absolute(Float) (.Pitch (Math|Rotator|BreakRotator (Math|Rotator|Delta(Rotator) (Variables|Default|GetOriginRotation) (Variables|Default|GetPostRotation))))) (Variables|Default|GetRecoilMaxThreshold) 3e+01 1.0 0.0) (Math|Float|MapRangeClamped (Math|Float|Absolute(Float) (.Pitch (Math|Rotator|BreakRotator (Math|Rotator|Delta(Rotator) (Variables|Default|GetOriginRotation) (Variables|Default|GetPostRotation))))) 0.0 (Variables|Default|GetRecoilMaxThreshold) 0.0 1.0))) (* _yawinput -3.0 (select (> (Math|Float|Absolute(Float) (.Pitch (Math|Rotator|BreakRotator (Math|Rotator|Delta(Rotator) (Variables|Default|GetOriginRotation) (Variables|Default|GetPostRotation))))) (Variables|Default|GetRecoilMaxThreshold)) (Math|Float|MapRangeClamped (Math|Float|Absolute(Float) (.Pitch (Math|Rotator|BreakRotator (Math|Rotator|Delta(Rotator) (Variables|Default|GetOriginRotation) (Variables|Default|GetPostRotation))))) (Variables|Default|GetRecoilMaxThreshold) 3e+01 1.0 0.0) (Math|Float|MapRangeClamped (Math|Float|Absolute(Float) (.Pitch (Math|Rotator|BreakRotator (Math|Rotator|Delta(Rotator) (Variables|Default|GetOriginRotation) (Variables|Default|GetPostRotation))))) 0.0 (Variables|Default|GetRecoilMaxThreshold) 0.0 1.0)))))))))
    (:Finished
      (switch Utilities|FlowControl|Switch|SwitchonETimelineDirection _direction
        (:Backward
          (CallFunction|ResetRecoil))))))

(event Custom|ResetRecoil
  (Utilities|FlowControl|Sequence
    (:then_0
      (Utilities|FlowControl|DoOnce false) ; enters at Reset
    )
    (:then_1
      (Utilities|FlowControl|DoOnce false) ; enters at Reset
    )))

(event Custom|ReloadEvent
  (CallFunction|Reload))

(fn ConstructionScript)

(fn ThreatTrace
  (params (ThreatValue :type Float%20%28double-precision%29))
  (bind _muzzle (Variables|Default|GetMuzzle))
  (bind _returnvalue (Transformation|GetWorldLocation _muzzle))
  (bind _outhit (Collision|SphereTraceByChannel _returnvalue (+ _returnvalue (* (Math|Vector|GetForwardVector (Transformation|GetWorldRotation _muzzle)) (Variables|Default|GetRange))) ThreatValue "TraceTypeQuery2" false (Utilities|Array|MakeArray (Components|GetOwner)) "None" true "(R=0.998619,G=0.094715,B=1.000000,A=1.000000)" "(R=0.000000,G=0.790609,B=1.000000,A=1.000000)"))
  (if (.bblockinghit _outhit)
    (bind _asenemy (Utilities|Casting|CastToEnemy (.hitactor _outhit)))
    (Default|Threathed _asenemy (.tracestart _outhit))))

(fn UpdatePlayerPitchandYaw
  (params (Val :type Float%20%28single-precision%29) (Val2 :type Float%20%28single-precision%29))
  (bind _returnvalue (Game|GetPlayerController 0))
  (Class|PlayerController|AddPitchInput _returnvalue Val)
  (Class|PlayerController|AddYawInput _returnvalue Val2))

(fn Reload
  (if (< (Variables|Default|GetAmmo) (Variables|Default|GetClipSize))
    (if (> (Variables|Default|GetMaxAmmo) (- (Variables|Default|GetClipSize) (Variables|Default|GetAmmo)))
      (Variables|Default|SetAmmoDifference (- (Variables|Default|GetClipSize) (Variables|Default|GetAmmo)))
      (Variables|Default|SetAmmo (+ (Variables|Default|GetAmmo) (Variables|Default|GetAmmoDifference)))
      (Variables|Default|SetMaxAmmo (- (Variables|Default|GetMaxAmmo) (Variables|Default|GetAmmoDifference)))
      (else
        (Variables|Default|SetAmmoDifference (- (Variables|Default|GetClipSize) (Variables|Default|GetAmmo)))
        (Variables|Default|SetAmmo (+ (Variables|Default|GetAmmo) (Variables|Default|GetMaxAmmo)))
        (Variables|Default|SetMaxAmmo 0)))))