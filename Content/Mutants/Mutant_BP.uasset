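; Mutant enemy character that loses health from player-character damage and exposes Attack and Roar events that play montages.
; On first reaching zero health, it ragdolls the mesh, disables capsule collision, plays a death sound, pauses animation, detaches its controller and sets a lifespan for delayed removal.
; Its audio component is randomly silenced at spawn and also stops on attack, roar or death.
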(event Custom|Roar
  (Animation|Montage|PlayMontage (Variables|Character|GetMesh) "/Game/Mutants/Anims/Mutant_Roaring_Montage.Mutant_Roaring_Montage"
    (:then
      (Audio|Components|Audio|Stop (Variables|Default|GetAudio)))))

(event EventBeginPlay
  (if (Math|Random|RandomBool)
    (Audio|Components|Audio|Stop (Variables|Default|GetAudio))))

(event Game|Damage|EventAnyDamage
  (params (Damage :type Float%20%28single-precision%29) (DamageType :type Damage%20Type%20Object%20Reference) (InstigatedBy :type Controller%20Object%20Reference) (DamageCauser :type Actor%20Object%20Reference))
  (Utilities|Casting|CastToUe4ASP_Character DamageCauser)
  (bind _output_get (Variables|Default|SetHealth (- (Variables|Default|GetHealth) Damage)))
  (if (<= _output_get 0.0)
    (Utilities|FlowControl|DoOnce false
      (:Completed
        (Physics|SetSimulatePhysics (Variables|Character|GetMesh) true)
        (Collision|SetCollisionEnabled (Variables|Collision|GetCapsuleComponent) "NoCollision")
        (Audio|PlaySoundatLocation "/Game/SFX/Skinwalker_sounds_death_1.Skinwalker_sounds_death_1" (Transformation|GetActorLocation) "0, 0, 0" 1.0 1.0 0.0 0 0 0 0)
        (Audio|Components|Audio|Stop (Variables|Default|GetAudio))
        (Variables|/Script/Engine.SkeletalMeshComponent|SetbPauseAnims (Variables|Character|GetMesh) true)
        (Class|Pawn|DetachfromControllerPendingDestroy)
        (Actor|SetLifeSpan 2e+01)))))

(event EventAttack
  (Animation|Montage|PlayMontage (Variables|Character|GetMesh) "/Game/Mutants/Anims/Mutant_Punch_Montage.Mutant_Punch_Montage"
    (:then
      (Audio|Components|Audio|Stop (Variables|Default|GetAudio)))))

(fn ConstructionScript)