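; Ammo magazine pickup for the AK47 that the player character collects by overlapping its Box.
; A DoOnce-guarded overlap plays a pickup sound, then adds random amounts to the character's TradeAmmo and to MaxAmmo on the AK47 child actor.
; It then refreshes the character's ammo HUD and destroys itself, stopping after the sound if the AK47 cast fails.
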(event OnComponentBeginOverlap(Box)
  (params (OverlappedComponent :type Primitive%20Component%20Object%20Reference) (OtherActor :type Actor%20Object%20Reference) (OtherComp :type Primitive%20Component%20Object%20Reference) (OtherBodyIndex :type Integer) (bFromSweep :type Boolean) (SweepResult :type Hit%20Result%20Structure%20%28by%20ref%29))
  (bind _asue_4asp_character (Utilities|Casting|CastToUe4ASP_Character OtherActor))
  (Utilities|FlowControl|DoOnce false
    (:Completed
      (Audio|PlaySound2D "/Game/SFX/Picking_Up_Ammo_Sound_Effect__Surviv_io.Picking_Up_Ammo_Sound_Effect__Surviv_io" 1.0 1.0 0.0 0 0)
      (bind _asak_47_bp (Utilities|Casting|CastToAk47_BP (Variables|/Script/Engine.ChildActorComponent|GetChildActor (Variables|/Game/AnimStarterPack/Ue4ASP_Character.Ue4ASP_Character_C|GetAk47_BP _asue_4asp_character))))
      (Variables|/Game/AnimStarterPack/Ue4ASP_Character.Ue4ASP_Character_C|SetTradeAmmo _asue_4asp_character (+ (Variables|/Game/AnimStarterPack/Ue4ASP_Character.Ue4ASP_Character_C|GetTradeAmmo _asue_4asp_character) (Math|Random|RandomIntegerinRange 0 5)))
      (Variables|/Game/Guns/Ak47/Ak47_BP.Ak47_BP_C|SetMaxAmmo _asak_47_bp (+ (Variables|/Game/Guns/Ak47/Ak47_BP.Ak47_BP_C|GetMaxAmmo _asak_47_bp) (Math|Random|RandomIntegerinRange 4 15)))
      (Default|SetAmmos (Variables|/Game/AnimStarterPack/Ue4ASP_Character.Ue4ASP_Character_C|GetAmmoHud _asue_4asp_character) (Variables|/Game/Guns/Ak47/Ak47_BP.Ak47_BP_C|GetAmmo (Variables|/Game/AnimStarterPack/Ue4ASP_Character.Ue4ASP_Character_C|GetAs%20Ak%2047%20BP _asue_4asp_character)) (Variables|/Game/Guns/Ak47/Ak47_BP.Ak47_BP_C|GetMaxAmmo (Variables|/Game/AnimStarterPack/Ue4ASP_Character.Ue4ASP_Character_C|GetAs%20Ak%2047%20BP _asue_4asp_character)))
      (Actor|DestroyActor))))

(event EventBeginPlay)

(event Collision|EventActorBeginOverlap
  (params (OtherActor :type Actor%20Object%20Reference)))

(event EventTick
  (params (DeltaSeconds :type Float%20%28single-precision%29)))

(fn ConstructionScript)