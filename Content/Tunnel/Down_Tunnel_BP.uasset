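; Downward tunnel segment of a procedurally chained metro, which decrements saved TunnelLevel on spawn.
; BeginPlay randomly spawns a cart, mutant or toxic smoke zone, kills lamps and adds dripping audio.
; Player triggers open the gate, spawning a random next tunnel and counting it in save, then close it, clean up hazards and destroy the segment.
; Toxic overlap loops gas-mask wear or radiation gain; the station roll is always overwritten.
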(event OnComponentBeginOverlap(Box)
  (params (OverlappedComponent :type Primitive%20Component%20Object%20Reference) (OtherActor :type Actor%20Object%20Reference) (OtherComp :type Primitive%20Component%20Object%20Reference) (OtherBodyIndex :type Integer) (bFromSweep :type Boolean) (SweepResult :type Hit%20Result%20Structure%20%28by%20ref%29))
  ;[0 1 0] OpenDoor-CreateNewTunnels
  (Utilities|Casting|CastToUe4ASP_Character OtherActor)
  (Utilities|FlowControl|DoOnce false
    (:Completed
      (CallFunction|OpentheDoor))))

(event OnComponentBeginOverlap(CloseDoorBox1)
  (params (OverlappedComponent :type Primitive%20Component%20Object%20Reference) (OtherActor :type Actor%20Object%20Reference) (OtherComp :type Primitive%20Component%20Object%20Reference) (OtherBodyIndex :type Integer) (bFromSweep :type Boolean) (SweepResult :type Hit%20Result%20Structure%20%28by%20ref%29))
  ;[0 1 0] DestoryTunnel
  (Utilities|Casting|CastToUe4ASP_Character OtherActor)
  (Utilities|FlowControl|DoOnce false
    (:Completed
      (Utilities|FlowControl|Delay 7.0)
      (Actor|DestroyActor))))

(event OnComponentBeginOverlap(CloseDoorBox)
  (params (OverlappedComponent :type Primitive%20Component%20Object%20Reference) (OtherActor :type Actor%20Object%20Reference) (OtherComp :type Primitive%20Component%20Object%20Reference) (OtherBodyIndex :type Integer) (bFromSweep :type Boolean) (SweepResult :type Hit%20Result%20Structure%20%28by%20ref%29))
  (bind _smokevar (Variables|Default|GetSmokeVar))
  (bind _radiatitonvar (Variables|Default|GetRadiatitonVar))
  (bind _drippingsoundvar (Variables|Default|GetDrippingSoundVar))
  ;[0 1 0] CloseDoor-Destroy
  (Utilities|Casting|CastToUe4ASP_Character OtherActor)
  (Utilities|FlowControl|DoOnce false
    (:Completed
      (CallFunction|ClosetheDoor)
      (Utilities|FlowControl|Delay 5.0)
      (Utilities|IsValid _drippingsoundvar
        (:Is%20Valid
          (Components|DestroyComponent _drippingsoundvar))
        (:Is%20Not%20Valid
          _))
      (Utilities|IsValid _smokevar
        (:Is%20Valid
          (Components|DestroyComponent _smokevar))
        (:Is%20Not%20Valid
          _))
      (Utilities|IsValid _radiatitonvar
        (:Is%20Valid
          (Components|DestroyComponent _radiatitonvar))
        (:Is%20Not%20Valid
          _))
      (for _array_element (Variables|Default|GetSpawnedObject)
        (Actor|DestroyActor _array_element)))))

(event OnComponentBeginOverlap(ToxicCol)
  (params (OverlappedComponent :type Primitive%20Component%20Object%20Reference) (OtherActor :type Actor%20Object%20Reference) (OtherComp :type Primitive%20Component%20Object%20Reference) (OtherBodyIndex :type Integer) (bFromSweep :type Boolean) (SweepResult :type Hit%20Result%20Structure%20%28by%20ref%29))
  ;[0 1 0] Toxic
  (if (Variables|Default|Gettoxiced)
    (bind _asue_4asp_character (Utilities|Casting|CastToUe4ASP_Character OtherActor))
    (Variables|Default|Setoutside false)
    (if (Variables|/Game/AnimStarterPack/Ue4ASP_Character.Ue4ASP_Character_C|GetGasMask _asue_4asp_character) :!label _label
      (Default|GasmaskRealibityDecrease _asue_4asp_character)
      (else
        (Default|RadiationIncrease _asue_4asp_character)))
    (Utilities|FlowControl|Delay 0.2)
    (if (not (Variables|Default|Getoutside))
      (goto _label))))

(event OnComponentEndOverlap(ToxicCol)
  (params (OverlappedComponent :type Primitive%20Component%20Object%20Reference) (OtherActor :type Actor%20Object%20Reference) (OtherComp :type Primitive%20Component%20Object%20Reference) (OtherBodyIndex :type Integer))
  ;[0 1 0] Toxic
  (if (Variables|Default|Gettoxiced)
    (Utilities|Casting|CastToUe4ASP_Character OtherActor)
    (Variables|Default|Setoutside true)))

(event Custom|OpenTheDoor
  ;[0 1 0] OpenDoor-CreateNewTunnels
  (Utilities|FlowControl|Sequence
    (:then_0
      (Audio|PlaySoundatLocation "/Game/SFX/NewGateSound.NewGateSound" (Transformation|GetWorldLocation (Variables|Default|GetGateDoor)) "0, 0, 0" 1.0 1.0 0.0 "/Game/SFX/Natural.Natural" 0 0 0)
      (bind _gateopening (Timeline|Timeline_0 Play)
        (:Update
          (Transformation|SetRelativeRotation (Variables|Default|GetGateDoor) (Math|Rotator|MakeRotator 0.0 0.0 (.z _gateopening)) false false))))
    (:then_1
      (if (== (Math|Random|RandomIntegerinRange 0 9) 9)
        (Variables|Default|SetMetroClass "/Game/Tunnel/Station_Tunnel_BP.Station_Tunnel_BP_C"))
      (Variables|Default|SetNumber (Math|Random|RandomIntegerinRange 0 3))
      (if (== (Variables|Default|GetNumber) 0)
        (Variables|Default|SetMetroClass "/Game/Tunnel/Normal_Tunnel_BP.Normal_Tunnel_BP_C")
        (Game|SpawnActorfromClass (Variables|Default|GetMetroClass) (Transformation|GetWorldTransform (Variables|Default|GetMetroSpawnPoint)) "Undefined" "SelectDefaultAtRuntime" 0 0 :!label _label)
        (bind _returnvalue (SaveGame|DoesSaveGameExist "metro"))
        (if _returnvalue
          (bind _returnvalue_2 (SaveGame|LoadGamefromSlot "metro"))
          (bind _asmetro_save_game (Utilities|Casting|CastToMetroSaveGame _returnvalue_2))
          (Math|Integer|IncrementInt (Variables|/Game/GameModes/MetroSaveGame.MetroSaveGame_C|GetMetroOpened _asmetro_save_game)
            (:%20%20
              (SaveGame|SaveGametoSlot _asmetro_save_game "metro")))
          (else
            (bind _returnvalue_3 (SaveGame|CreateSaveGameObject "/Game/GameModes/MetroSaveGame.MetroSaveGame_C"))
            (Math|Integer|IncrementInt (Variables|/Game/GameModes/MetroSaveGame.MetroSaveGame_C|GetMetroOpened _returnvalue_3)
              (:%20%20
                (SaveGame|SaveGametoSlot _returnvalue_3 "metro")))))
        (elif (== (Variables|Default|GetNumber) 1)
          (Variables|Default|SetMetroClass "/Game/Tunnel/Left_Tunnel_BP.Left_Tunnel_BP_C")
          (goto _label)
          (elif (== (Variables|Default|GetNumber) 2)
            (Variables|Default|SetMetroClass "/Game/Tunnel/Right_Tunnel_BP.Right_Tunnel_BP_C")
            (goto _label)
            (elif (== (Variables|Default|GetNumber) 3)
              (Variables|Default|SetMetroClass "/Game/Tunnel/Up_Tunnel_BP.Up_Tunnel_BP_C")
              (goto _label))))))))

(event Custom|CloseTheDoor
  (bind _gatedoor (Variables|Default|GetGateDoor))
  ;[0 1 0] OpenDoor-CreateNewTunnels
  (Audio|PlaySoundatLocation "/Game/SFX/NewGateSound.NewGateSound" (Transformation|GetWorldLocation _gatedoor) "0, 0, 0" 1.0 1.0 0.0 "/Game/SFX/Natural.Natural" 0 0 0)
  (bind _gateopening (Timeline|Timeline_0 Reverse)
    (:Update
      (Transformation|SetRelativeRotation _gatedoor (Math|Rotator|MakeRotator 0.0 0.0 (.z _gateopening)) false false))))

(event Custom|RandomEvent
  (bind _returnvalue (Math|Random|RandomBool))
  (bind _toxicdeath (Variables|Default|GetToxicDeath))
  (bind _cartplacegood (Variables|Default|GetCartPlaceGood))
  (bind _cartplacebad (Variables|Default|GetCartPlaceBad))
  (bind _toxic (Variables|Default|GetToxic))
  (bind _returnvalue_2 (Transformation|GetWorldTransform _toxic))
  (bind _returnvalue_3 (Transformation|GetWorldTransform _cartplacebad))
  (bind _returnvalue_4 (Transformation|GetWorldTransform _cartplacegood))
  (bind _returnvalue_5 (Transformation|GetWorldTransform _toxicdeath))
  (bind _returnvalue_6 (Math|Transform|SelectTransform _returnvalue_4 _returnvalue_3 _returnvalue))
  ;[0 1 0] RandomEvent
  (if (not (Math|Random|RandomBool))
    (if (Math|Random|RandomBool)
      (bind _returnvalue_7 (Game|SpawnActorfromClass "/Game/Models/Cart/Cart_BP.Cart_BP_C" (Math|Transform|MakeTransform (Math|Vector|MakeVector (.x (.location _returnvalue_6)) (.y (.location _returnvalue_6)) (.z (.location _returnvalue_6))) (.rotation _returnvalue_6) (.scale _returnvalue_6)) "Undefined" "OverrideRootScale" 0 0))
      (Utilities|Array|Add (Variables|Default|GetSpawnedObject) _returnvalue_7)
      (if (Variables|/Game/Models/Cart/Cart_BP.Cart_BP_C|Getdummy _returnvalue_7)
        (bind _outactors (Actor|GetAllActorsOfClass "/Game/Models/Dummy/Dummy.Dummy_C"))
        (Utilities|Array|Add (Variables|Default|GetSpawnedObject) (Utilities|Array|Get(acopy) _outactors)))
      (elif (Math|Random|RandomBool)
        (bind _returnvalue_8 (Game|SpawnActorfromClass "/Game/Mutants/Mutant_BP.Mutant_BP_C" (Transformation|GetWorldTransform (Variables|Default|GetMutantSpawner1)) "Undefined" "MultiplyWithRoot" 0 0))
        (Utilities|Array|Add (Variables|Default|GetSpawnedObject) _returnvalue_8)
        (else
          (bind _returnvalue_9 (Niagara|SpawnSystematLocation "/Game/VFX/Smoke_N.Smoke_N" (.location _returnvalue_2) (.rotation _returnvalue_2) "1.000000,1.000000,1.000000" false))
          (Variables|Default|SetSmokeVar _returnvalue_9)
          (bind _returnvalue_10 (Audio|SpawnSoundatLocation "/Game/SFX/Extreme_Radiation_sound_-_extreme__mp3cut_net_.Extreme_Radiation_sound_-_extreme__mp3cut_net_" (.location _returnvalue_2) "0, 0, 0" 1.0 1.0 0.0 "/Game/SFX/Atmosphere.Atmosphere" 0))
          (Variables|Default|SetRadiatitonVar _returnvalue_10)
          (Variables|Default|Settoxiced true)
          (if (Math|Random|RandomBool)
            (bind _returnvalue_11 (Game|SpawnActorfromClass "/Game/Models/Dummy/Dummy.Dummy_C" (Math|Transform|MakeTransform (Math|Vector|MakeVector (.x (.location _returnvalue_5)) (.y (.location _returnvalue_5)) (.z (.location _returnvalue_5))) (.rotation _returnvalue_5) (.scale _returnvalue_5)) "Undefined" "OverrideRootScale" 0 0))
            (Utilities|Array|Add (Variables|Default|GetSpawnedObject) _returnvalue_11)))))))

(event EventBeginPlay
  ;[0 1 0] BeginPlay
  (Utilities|FlowControl|Sequence
    (:then_0
      (bind _returnvalue (SaveGame|DoesSaveGameExist "tunnel"))
      (if _returnvalue
        (bind _returnvalue_2 (SaveGame|LoadGamefromSlot "tunnel"))
        (bind _asmetro_save_game (Utilities|Casting|CastToMetroSaveGame _returnvalue_2))
        (Math|Integer|DecrementInt (Variables|/Game/GameModes/MetroSaveGame.MetroSaveGame_C|GetTunnelLevel _asmetro_save_game)
          (:%20%20
            (SaveGame|SaveGametoSlot _asmetro_save_game "tunnel")))
        (else
          (bind _returnvalue_3 (SaveGame|CreateSaveGameObject "/Game/GameModes/MetroSaveGame.MetroSaveGame_C"))
          (Math|Integer|DecrementInt (Variables|/Game/GameModes/MetroSaveGame.MetroSaveGame_C|GetTunnelLevel _returnvalue_3)
            (:%20%20
              (SaveGame|SaveGametoSlot _returnvalue_3 "tunnel"))))))
    (:then_1
      (CallFunction|RandomEvent)
      (Utilities|FlowControl|Sequence
        (:then_0
          (if (Math|Random|RandomBool)
            (if (Math|Random|RandomBool)
              (Components|DestroyComponent (Variables|Default|GetPointLight2))
              (Rendering|Material|SetMaterial (Variables|Default|GetLamp3) 0 "/Game/Tunnel/Meshes/Materials/Lamp/Lamp_Mat_Inst_Off.Lamp_Mat_Inst_Off"))))
        (:then_1
          (if (Math|Random|RandomBool)
            (if (Math|Random|RandomBool)
              (Components|DestroyComponent (Variables|Default|GetPointLight3))
              (Rendering|Material|SetMaterial (Variables|Default|GetLamp4) 0 "/Game/Tunnel/Meshes/Materials/Lamp/Lamp_Mat_Inst_Off.Lamp_Mat_Inst_Off"))))
        (:then_2
          (if (Math|Random|RandomBool)
            (if (Math|Random|RandomBool)
              (Components|DestroyComponent (Variables|Default|GetPointLight1))
              (Rendering|Material|SetMaterial (Variables|Default|GetLamp2) 0 "/Game/Tunnel/Meshes/Materials/Lamp/Lamp_Mat_Inst_Off.Lamp_Mat_Inst_Off"))))
        (:then_3
          (if (Math|Random|RandomBool)
            (if (Math|Random|RandomBool)
              (Components|DestroyComponent (Variables|Default|GetPointLight))
              (Rendering|Material|SetMaterial (Variables|Default|GetLamp1) 0 "/Game/Tunnel/Meshes/Materials/Lamp/Lamp_Mat_Inst_Off.Lamp_Mat_Inst_Off"))))
        (:then_4
          (if (Math|Random|RandomBool)
            (if (Math|Random|RandomBool)
              (Components|DestroyComponent (Variables|Default|GetPointLight4))
              (Rendering|Material|SetMaterial (Variables|Default|GetLamp5) 0 "/Game/Tunnel/Meshes/Materials/Lamp/Lamp_Mat_Inst_Off.Lamp_Mat_Inst_Off"))))))
    (:then_2
      (if (Math|Random|RandomBool)
        (bind _returnvalue_4 (Audio|SpawnSoundatLocation "/Game/SFX/dripping-water-in-cave-114694__mp3cut_net___1_.dripping-water-in-cave-114694__mp3cut_net___1_" (Transformation|GetWorldLocation (Variables|Default|GetTunnel)) "0, 0, 0" 1.0 1.0 0.0 "/Game/SFX/Atmosphere.Atmosphere" 0 false))
        (Variables|Default|SetDrippingSoundVar _returnvalue_4)))))

(fn ConstructionScript)