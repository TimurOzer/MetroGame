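; Mutant AI enemy character whose starting health rises with the MetroOpened value from the "metro" save.
; Only damage caused by the Ue4ASP_Character reduces health, with a hit sound.
; Death runs once: it ragdolls the mesh, detaches the controller, increments the Rhino count in the "bounty" save, then expires after a delay.
; Attack plays a random swipe or punch montage, while Scream halts walking until its roar montage completes.
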(event Custom|Scream
  (bind _charactermovement (Variables|Character|GetCharacterMovement))
  (Animation|Montage|PlayMontage (Variables|Character|GetMesh) "/Game/Ai/Mutant/Anims/Mutant_Roaring__1__Montage.Mutant_Roaring__1__Montage"
    (:then
      (Variables|/Script/Engine.CharacterMovementComponent|SetMaxWalkSpeed _charactermovement 0.0))
    (:OnCompleted
      (Variables|/Script/Engine.CharacterMovementComponent|SetMaxWalkSpeed _charactermovement 1.5e+02))))

(event EventBeginPlay
  (bind _returnvalue (SaveGame|DoesSaveGameExist "metro"))
  (if _returnvalue
    (bind _returnvalue_2 (SaveGame|LoadGamefromSlot "metro"))
    (bind _asmetro_save_game (Utilities|Casting|CastToMetroSaveGame _returnvalue_2))
    (Variables|Default|SetHealth (+ (Variables|Default|GetHealth) (Math|Conversions|ToFloat(Integer) (* (Variables|/Game/GameModes/MetroSaveGame.MetroSaveGame_C|GetMetroOpened _asmetro_save_game) 5))))
    (else
      (bind _returnvalue_3 (SaveGame|CreateSaveGameObject "/Game/GameModes/MetroSaveGame.MetroSaveGame_C"))
      (Variables|Default|SetHealth (+ (Variables|Default|GetHealth) (Math|Conversions|ToFloat(Integer) (* (Variables|/Game/GameModes/MetroSaveGame.MetroSaveGame_C|GetMetroOpened _returnvalue_3) 5)))))))

(event Collision|EventActorBeginOverlap
  (params (OtherActor :type Actor%20Object%20Reference)))

(event EventTick
  (params (DeltaSeconds :type Float%20%28single-precision%29)))

(event EventAttack
  (Animation|Montage|PlayMontage (Variables|Character|GetMesh) (Utilities|Select :Index (Math|Random|RandomIntegerinRange 0 1) :Option%200 "/Game/Ai/Mutant/Anims/Mutant_Swiping__1__Montage.Mutant_Swiping__1__Montage" :Option%201 "/Game/Ai/Mutant/Anims/Mutant_Punch__1__Montage.Mutant_Punch__1__Montage")))

(event Game|Damage|EventAnyDamage
  (params (Damage :type Float%20%28single-precision%29) (DamageType :type Damage%20Type%20Object%20Reference) (InstigatedBy :type Controller%20Object%20Reference) (DamageCauser :type Actor%20Object%20Reference))
  (Utilities|Casting|CastToUe4ASP_Character DamageCauser)
  (bind _output_get (Variables|Default|SetHealth (- (Variables|Default|GetHealth) Damage)))
  (Audio|PlaySoundatLocation "/Game/SFX/Mutant3/Mutant3Hit.Mutant3Hit" (Transformation|GetActorLocation) "0, 0, 0" 1.0 1.0 0.0 0 0 0 0)
  (Utilities|FlowControl|Delay 0.1)
  (if (<= _output_get 0.0)
    (Utilities|FlowControl|DoOnce false
      (:Completed
        (Audio|PlaySoundatLocation "/Game/SFX/Mutant3/Mutant3Death.Mutant3Death" (Transformation|GetActorLocation) "0, 0, 0" 1.0 1.0 0.0 0 0 0 0)
        (Physics|SetSimulatePhysics (Variables|Character|GetMesh) true)
        (Collision|SetCollisionEnabled (Variables|Collision|GetCapsuleComponent) "NoCollision")
        (Variables|/Script/Engine.SkeletalMeshComponent|SetbPauseAnims (Variables|Character|GetMesh) true)
        (Class|Pawn|DetachfromControllerPendingDestroy)
        (bind _returnvalue (SaveGame|DoesSaveGameExist "bounty"))
        (if _returnvalue
          (bind _returnvalue_2 (SaveGame|LoadGamefromSlot "bounty"))
          (bind _asmetro_save_game (Utilities|Casting|CastToMetroSaveGame _returnvalue_2))
          (Math|Integer|IncrementInt (Variables|/Game/GameModes/MetroSaveGame.MetroSaveGame_C|GetRhino _asmetro_save_game)
            (:%20%20
              (SaveGame|SaveGametoSlot _asmetro_save_game "bounty")))
          (else
            (bind _returnvalue_3 (SaveGame|CreateSaveGameObject "/Game/GameModes/MetroSaveGame.MetroSaveGame_C"))
            (bind _asmetro_save_game_2 (Utilities|Casting|CastToMetroSaveGame _returnvalue_3))
            (Math|Integer|IncrementInt (Variables|/Game/GameModes/MetroSaveGame.MetroSaveGame_C|GetRhino _asmetro_save_game_2)
              (:%20%20
                (SaveGame|SaveGametoSlot _asmetro_save_game_2 "bounty")))))
        (Actor|SetLifeSpan 2e+01)))))

(fn ConstructionScript)