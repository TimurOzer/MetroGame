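; Drake is an AI enemy character with scream and attack events that play montages, and health that drops only from damage caused by the player character class.
; Hits play impact and delayed pain sounds.
; At zero health, a one-time death sequence ragdolls the mesh, disables capsule collision and detaches the controller.
; It then increments the Drake count in the "bounty" save slot, creating the save if absent, and sets a despawn lifespan.
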(event Custom|Scream
  (Animation|Montage|PlayMontage (Variables|Character|GetMesh) "/Game/Ai/Drake/Anims/Zombie_Scream_Montage.Zombie_Scream_Montage"))

(event EventBeginPlay)

(event Collision|EventActorBeginOverlap
  (params (OtherActor :type Actor%20Object%20Reference)))

(event EventTick
  (params (DeltaSeconds :type Float%20%28single-precision%29)))

(event EventAttack
  (Animation|Montage|PlayMontage (Variables|Character|GetMesh) "/Game/Ai/Drake/Anims/Mutant_Swiping_Montage.Mutant_Swiping_Montage"))

(event Game|Damage|EventAnyDamage
  (params (Damage :type Float%20%28single-precision%29) (DamageType :type Damage%20Type%20Object%20Reference) (InstigatedBy :type Controller%20Object%20Reference) (DamageCauser :type Actor%20Object%20Reference))
  (bind _returnvalue (Transformation|GetActorLocation))
  (Utilities|Casting|CastToUe4ASP_Character DamageCauser)
  (bind _output_get (Variables|Default|SetHealth (- (Variables|Default|GetHealth) Damage)))
  (Audio|PlaySoundatLocation "/Game/SFX/Mutant4/Mutant4Hit.Mutant4Hit" _returnvalue "0, 0, 0" 1.0 1.0 0.0 0 0 0 0)
  (Utilities|FlowControl|Delay 0.1)
  (Audio|PlaySoundatLocation "/Game/SFX/Mutant4/Mutant4Pain.Mutant4Pain" _returnvalue "0, 0, 0" 1.0 1.0 0.0 0 0 0 0)
  (if (<= _output_get 0.0)
    (Utilities|FlowControl|DoOnce false
      (:Completed
        (Audio|PlaySoundatLocation "/Game/SFX/Mutant4/MutantDeath.MutantDeath" (Transformation|GetActorLocation) "0, 0, 0" 1.0 1.0 0.0 0 0 0 0)
        (Physics|SetSimulatePhysics (Variables|Character|GetMesh) true)
        (Collision|SetCollisionEnabled (Variables|Collision|GetCapsuleComponent) "NoCollision")
        (Variables|/Script/Engine.SkeletalMeshComponent|SetbPauseAnims (Variables|Character|GetMesh) true)
        (Class|Pawn|DetachfromControllerPendingDestroy)
        (bind _returnvalue_2 (SaveGame|DoesSaveGameExist "bounty"))
        (if _returnvalue_2
          (bind _returnvalue_3 (SaveGame|LoadGamefromSlot "bounty"))
          (bind _asmetro_save_game (Utilities|Casting|CastToMetroSaveGame _returnvalue_3))
          (Math|Integer|IncrementInt (Variables|/Game/GameModes/MetroSaveGame.MetroSaveGame_C|GetDrake _asmetro_save_game)
            (:%20%20
              (SaveGame|SaveGametoSlot _asmetro_save_game "bounty")))
          (else
            (bind _returnvalue_4 (SaveGame|CreateSaveGameObject "/Game/GameModes/MetroSaveGame.MetroSaveGame_C"))
            (bind _asmetro_save_game_2 (Utilities|Casting|CastToMetroSaveGame _returnvalue_4))
            (Math|Integer|IncrementInt (Variables|/Game/GameModes/MetroSaveGame.MetroSaveGame_C|GetDrake _asmetro_save_game_2)
              (:%20%20
                (SaveGame|SaveGametoSlot _asmetro_save_game_2 "bounty")))))
        (Actor|SetLifeSpan 2e+01)))))

(fn ConstructionScript)