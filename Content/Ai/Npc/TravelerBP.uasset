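; Traveler NPC that shows a Traveler widget when interacted with and can be taken along to follow the player.
; TakeHim sets the Traveler flag in the MetroSaveGame "bounty" slot, creating the save if none exists.
; It then tells its TravelerController AI to follow the player.
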(event Custom|TakeHim
  (bind _returnvalue (SaveGame|DoesSaveGameExist "bounty"))
  (if _returnvalue
    (bind _returnvalue_2 (SaveGame|LoadGamefromSlot "bounty"))
    (bind _asmetro_save_game (Utilities|Casting|CastToMetroSaveGame _returnvalue_2))
    (Variables|/Game/GameModes/MetroSaveGame.MetroSaveGame_C|SetTraveler _asmetro_save_game true)
    (SaveGame|SaveGametoSlot _asmetro_save_game "bounty")
    (else
      (bind _returnvalue_3 (SaveGame|CreateSaveGameObject "/Game/GameModes/MetroSaveGame.MetroSaveGame_C"))
      (Variables|/Game/GameModes/MetroSaveGame.MetroSaveGame_C|SetTraveler _returnvalue_3 true)
      (SaveGame|SaveGametoSlot _returnvalue_3 "bounty")))
  (bind _astraveler_controller (Utilities|Casting|CastToTravelerController (AI|GetAIController self)))
  (Default|FollowPlayer _astraveler_controller))

(event EventBeginPlay)

(event Collision|EventActorBeginOverlap
  (params (OtherActor :type Actor%20Object%20Reference)))

(event EventTick
  (params (DeltaSeconds :type Float%20%28single-precision%29)))

(event EventInteractingObject
  (bind _returnvalue (UserInterface|CreateWidget "/Game/UI/Traveler.Traveler_C"))
  (UserInterface|Viewport|AddtoViewport _returnvalue 0))

(fn ConstructionScript)