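; Parasite mutant enemy with montage-driven attack and roar events, and a Darkside variant that swaps material and teleports onto the player when attacking or hit.
; On spawn it plays a biting montage and adds health scaled by MetroOpened from the "metro" save.
; Only damage caused by the player character class counts.
; Death ragdolls it, detaches its controller, increments the ParasiteMutant count in the "bounty" save and sets a lifespan.
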(event Custom|Roar
  (Animation|Montage|PlayMontage (Variables|Character|GetMesh) "/Game/Ai/Parasite/Anims/Mutant_Roaring_Montage.Mutant_Roaring_Montage"))

(event Custom|DarkParasite
  (Rendering|Material|SetMaterial (Variables|Character|GetMesh) 0 "/Game/Ai/Parasite/parasitezombie_Material_2.parasitezombie_Material_2")
  (Variables|Default|Setdarkside true))

(event EventBeginPlay
  (Animation|Montage|PlayMontage (Variables|Character|GetMesh) "/Game/Ai/Parasite/Anims/Zombie_Biting__1__Montage.Zombie_Biting__1__Montage"
    (:then
      (bind _returnvalue (SaveGame|DoesSaveGameExist "metro"))
      (if _returnvalue
        (bind _returnvalue_2 (SaveGame|LoadGamefromSlot "metro"))
        (bind _asmetro_save_game (Utilities|Casting|CastToMetroSaveGame _returnvalue_2))
        (Variables|Default|SetHealth (+ (Variables|Default|GetHealth) (Math|Conversions|ToFloat(Integer) (* (Variables|/Game/GameModes/MetroSaveGame.MetroSaveGame_C|GetMetroOpened _asmetro_save_game) 5))))
        (else
          (bind _returnvalue_3 (SaveGame|CreateSaveGameObject "/Game/GameModes/MetroSaveGame.MetroSaveGame_C"))
          (Variables|Default|SetHealth (+ (Variables|Default|GetHealth) (Math|Conversions|ToFloat(Integer) (* (Variables|/Game/GameModes/MetroSaveGame.MetroSaveGame_C|GetMetroOpened _returnvalue_3) 5)))))))))

(event Game|Damage|EventAnyDamage
  (params (Damage :type Float%20%28single-precision%29) (DamageType :type Damage%20Type%20Object%20Reference) (InstigatedBy :type Controller%20Object%20Reference) (DamageCauser :type Actor%20Object%20Reference))
  (Utilities|Casting|CastToUe4ASP_Character DamageCauser)
  (bind _output_get (Variables|Default|SetHealth (- (Variables|Default|GetHealth) Damage)))
  (if (Variables|Default|Getdarkside)
    (Transformation|Teleport (Transformation|GetActorLocation (Game|GetPlayerCharacter 0)) "0, 0, 0"))
  (Audio|PlaySoundatLocation "/Game/SFX/Mutant2/Mutant2Pain.Mutant2Pain" (Transformation|GetActorLocation) "0, 0, 0" 1.0 1.0 0.0 0 0 0 0)
  (Utilities|FlowControl|Delay 0.1)
  (if (<= _output_get 0.0)
    (Utilities|FlowControl|DoOnce false
      (:Completed
        (Audio|PlaySoundatLocation "/Game/SFX/Mutant2/Mutant2Die.Mutant2Die" (Transformation|GetActorLocation) "0, 0, 0" 1.0 1.0 0.0 0 0 0 0)
        (Physics|SetSimulatePhysics (Variables|Character|GetMesh) true)
        (Collision|SetCollisionEnabled (Variables|Collision|GetCapsuleComponent) "NoCollision")
        (Audio|PlaySoundatLocation "/Game/SFX/Skinwalker_sounds_death_1.Skinwalker_sounds_death_1" (Transformation|GetActorLocation) "0, 0, 0" 1.0 1.0 0.0 0 0 0 0)
        (Variables|/Script/Engine.SkeletalMeshComponent|SetbPauseAnims (Variables|Character|GetMesh) true)
        (Class|Pawn|DetachfromControllerPendingDestroy)
        (bind _returnvalue (SaveGame|DoesSaveGameExist "bounty"))
        (if _returnvalue
          (bind _returnvalue_2 (SaveGame|LoadGamefromSlot "bounty"))
          (bind _asmetro_save_game (Utilities|Casting|CastToMetroSaveGame _returnvalue_2))
          (Math|Integer|IncrementInt (Variables|/Game/GameModes/MetroSaveGame.MetroSaveGame_C|GetParasiteMutant _asmetro_save_game)
            (:%20%20
              (SaveGame|SaveGametoSlot _asmetro_save_game "bounty")))
          (else
            (bind _returnvalue_3 (SaveGame|CreateSaveGameObject "/Game/GameModes/MetroSaveGame.MetroSaveGame_C"))
            (bind _asmetro_save_game_2 (Utilities|Casting|CastToMetroSaveGame _returnvalue_3))
            (Math|Integer|IncrementInt (Variables|/Game/GameModes/MetroSaveGame.MetroSaveGame_C|GetParasiteMutant _asmetro_save_game_2)
              (:%20%20
                (SaveGame|SaveGametoSlot _asmetro_save_game_2 "bounty")))))
        (Actor|SetLifeSpan 2e+01)))))

(event EventAttack
  (Animation|Montage|PlayMontage (Variables|Character|GetMesh) "/Game/Ai/Parasite/Anims/Mutant_Punch_Montage.Mutant_Punch_Montage"
    (:then
      (if (Variables|Default|Getdarkside)
        (Transformation|Teleport (Transformation|GetActorLocation (Game|GetPlayerCharacter 0)) "0, 0, 0")))))

(fn ConstructionScript)