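; Interactable cart that randomly hides a spawned Dummy, revealed when the cart is opened.
; On BeginPlay a coin flip decides whether a Dummy spawns at DummyPlace, with its mesh collision set to physics only.
; Interacting calls OpenDoor, where a timeline rotates the cart's SkeletalMesh.
; When the timeline finishes, the Box collision is disabled and any spawned Dummy gets query and physics collision.
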(event Custom|OpenDoor
  (bind _newtrack_0 (Timeline|Timeline_0 Play)
    (:Update
      (Transformation|SetRelativeRotation (Variables|Default|GetSkeletalMesh) (Math|Rotator|MakeRotator (.x _newtrack_0) (.y _newtrack_0) (.z _newtrack_0)) false false))
    (:Finished
      (Collision|SetCollisionEnabled (Variables|Default|GetBox) "NoCollision")
      (Utilities|IsValid (stale EventBeginPlay _returnvalue)
        (:Is%20Valid
          (Collision|SetCollisionEnabled (Variables|/Game/Models/Dummy/Dummy.Dummy_C|GetSkeletalMesh (stale EventBeginPlay _returnvalue)) "QueryAndPhysics"))))))

(event EventBeginPlay
  (if (Math|Random|RandomBool)
    (bind _returnvalue (Game|SpawnActorfromClass "/Game/Models/Dummy/Dummy.Dummy_C" (Transformation|GetWorldTransform (Variables|Default|GetDummyPlace)) "Undefined" 0 0))
    (Variables|Default|Setdummy true)
    (Collision|SetCollisionEnabled (Variables|/Game/Models/Dummy/Dummy.Dummy_C|GetSkeletalMesh _returnvalue) "PhysicsOnly")))

(event EventInteractingObject
  (CallFunction|OpenDoor))

(fn ConstructionScript)