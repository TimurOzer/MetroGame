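; Bulkhead light fixture Blueprint pairing a Light mesh with a RectLight.
; Its construction script makes a dynamic instance of the mesh's second material slot and randomizes the Speed parameter, varying each placed copy.
; BeginPlay does nothing; a disconnected graph would randomly choose lit or unlit material with matching RectLight visibility, weighted toward lit, but never runs.
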(event EventBeginPlay)

(fn ConstructionScript
  (bind _light (Variables|Default|GetLight))
  (bind _returnvalue (Rendering|Material|CreateDynamicMaterialInstance _light 1 (Rendering|Material|GetMaterial _light 1) "None" :!class /Script/Engine.PrimitiveComponent))
  (Rendering|Material|SetScalarParameterValue _returnvalue "Speed" (Math|Random|RandomFloatinRange 0.01 1.0) :!class /Script/Engine.MaterialInstanceDynamic))