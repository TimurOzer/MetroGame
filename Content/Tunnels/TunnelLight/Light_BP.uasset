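; Tunnel light Blueprint that pairs a Light mesh with a RectLight.
; On BeginPlay it reads the "raytrace" save slot and gives the RectLight a smaller attenuation radius when Lumen is on, a larger one otherwise or without a save.
; The construction script creates a dynamic material with a random Speed parameter to vary each instance.
; An unconnected graph for randomly switching lights off never runs.
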(event EventBeginPlay
  (bind _returnvalue (SaveGame|DoesSaveGameExist "raytrace"))
  (if _returnvalue
    (bind _returnvalue_2 (SaveGame|LoadGamefromSlot "raytrace"))
    (bind _asmetro_save_game (Utilities|Casting|CastToMetroSaveGame _returnvalue_2))
    (if (Variables|/Game/GameModes/MetroSaveGame.MetroSaveGame_C|GetLumen _asmetro_save_game)
      (Variables|Default|SetNew%20Radius 9e+02)
      (else
        (Variables|Default|SetNew%20Radius 1.1e+03)))
    (else
      (Variables|Default|SetNew%20Radius 1.1e+03)))
  (Rendering|Lighting|SetAttenuationRadius (Variables|Default|GetRectLight) (Variables|Default|GetNew%20Radius)))

(fn ConstructionScript
  (bind _light (Variables|Default|GetLight))
  (bind _returnvalue (Rendering|Material|CreateDynamicMaterialInstance _light 1 (Rendering|Material|GetMaterial _light 1) "None" :!class /Script/Engine.PrimitiveComponent))
  (Rendering|Material|SetScalarParameterValue _returnvalue "Speed" (Math|Random|RandomFloatinRange 0.1 1.0) :!class /Script/Engine.MaterialInstanceDynamic))