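; Wagon Blueprint that rides along a referenced Tunnel's spline from start to end when play begins.
; A timeline, with play rate set from TimeToComplete, drives an alpha that maps to distance along the spline.
; Each update moves the actor to that point with a fixed world-space Y and Z offset and matches the spline's rotation.
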(event Custom|Move
  (bind _tunnel (Variables|Default|GetTunnel))
  (bind _spline (Variables|/Game/Tunnels/TunnelCreator.TunnelCreator_C|GetSpline _tunnel))
  (Components|Timeline|SetPlayRate (Variables|Default|GetMoveObjectT) (/ 1.0 (Variables|Default|GetTimeToComplete)))
  (bind _movetrack (Timeline|MoveObjectT Play)
    (:Update
      (Transformation|SetActorTransform (Math|Transform|MakeTransform (Math|Vector|MakeVector (.x (Spline|GetLocationatDistanceAlongSpline _spline (Math|Float|Lerp 0.0 (Spline|GetSplineLength _spline) _movetrack) "World")) (+ (.y (Spline|GetLocationatDistanceAlongSpline _spline (Math|Float|Lerp 0.0 (Spline|GetSplineLength _spline) _movetrack) "World")) 1e+02) (- (.z (Spline|GetLocationatDistanceAlongSpline _spline (Math|Float|Lerp 0.0 (Spline|GetSplineLength _spline) _movetrack) "World")) 115.0)) (Spline|GetRotationatDistanceAlongSpline _spline (Math|Float|Lerp 0.0 (Spline|GetSplineLength _spline) _movetrack) "World") "1.000000,1.000000,1.000000")))))

(event EventBeginPlay
  (CallFunction|Move))

(fn ConstructionScript)