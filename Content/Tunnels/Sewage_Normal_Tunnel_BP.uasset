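; Sewage tunnel segment of an endlessly chained metro that rolls a random event on BeginPlay: nothing, cart, creature, toxic gas or save-and-load into StationLevel.
; Overlap triggers open the gate, spawn a random next tunnel (up/down limited by saved TunnelLevel) and increment a saved counter.
; Later triggers close the gate, clean up spawned content and destroy the segment.
; Gas loops damage to gas mask reliability, or adds radiation without one.
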(event OnComponentBeginOverlap(Box)
  (params (OverlappedComponent :type Primitive%20Component%20Object%20Reference) (OtherActor :type Actor%20Object%20Reference) (OtherComp :type Primitive%20Component%20Object%20Reference) (OtherBodyIndex :type Integer) (bFromSweep :type Boolean) (SweepResult :type Hit%20Result%20Structure%20%28by%20ref%29))
  ;[0 1 0] OpenDoor-CreateNewTunnels
  (Utilities|Casting|CastToUe4ASP_Character OtherActor)
  (Utilities|FlowControl|DoOnce false
    (:Completed
      (CallFunction|OpentheDoor))))

(event OnComponentBeginOverlap(CloseDoorBox1)
  (params (OverlappedComponent :type Primitive%20Component%20Object%20Reference) (OtherActor :type Actor%20Object%20Reference) (OtherComp :type Primitive%20Component%20Object%20Reference) (OtherBodyIndex :type Integer) (bFromSweep :type Boolean) (SweepResult :type Hit%20Result%20Structure%20%28by%20ref%29))
  ;[0 1 0] DestoryTunnel
  (Utilities|Casting|CastToUe4ASP_Character OtherActor)
  (Utilities|FlowControl|DoOnce false
    (:Completed
      (Utilities|FlowControl|Delay 7.0)
      (Actor|DestroyActor))))

(event OnComponentBeginOverlap(CloseDoorBox)
  (params (OverlappedComponent :type Primitive%20Component%20Object%20Reference) (OtherActor :type Actor%20Object%20Reference) (OtherComp :type Primitive%20Component%20Object%20Reference) (OtherBodyIndex :type Integer) (bFromSweep :type Boolean) (SweepResult :type Hit%20Result%20Structure%20%28by%20ref%29))
  (bind _smokevar (Variables|Default|GetSmokeVar))
  (bind _radiatitonvar (Variables|Default|GetRadiatitonVar))
  (bind _drippingsoundvar (Variables|Default|GetDrippingSoundVar))
  ;[0 1 0] CloseDoor-Destroy
  (Utilities|Casting|CastToUe4ASP_Character OtherActor)
  (Utilities|FlowControl|DoOnce false
    (:Completed
      (CallFunction|ClosetheDoor)
      (Utilities|FlowControl|Delay 5.0)
      (Utilities|IsValid _drippingsoundvar
        (:Is%20Valid
          (Components|DestroyComponent _drippingsoundvar))
        (:Is%20Not%20Valid
          _))
      (Utilities|IsValid _smokevar
        (:Is%20Valid
          (Components|DestroyComponent _smokevar))
        (:Is%20Not%20Valid
          _))
      (Utilities|IsValid _radiatitonvar
        (:Is%20Valid
          (Components|DestroyComponent _radiatitonvar))
        (:Is%20Not%20Valid
          _))
      (for _array_element (Variables|Default|GetSpawnedObject)
        (Actor|DestroyActor _array_element)))))

(event OnComponentBeginOverlap(ToxicCol)
  (params (OverlappedComponent :type Primitive%20Component%20Object%20Reference) (OtherActor :type Actor%20Object%20Reference) (OtherComp :type Primitive%20Component%20Object%20Reference) (OtherBodyIndex :type Integer) (bFromSweep :type Boolean) (SweepResult :type Hit%20Result%20Structure%20%28by%20ref%29))
  ;[0 1 0] Toxic
  (if (Variables|Default|Gettoxiced)
    (bind _asue_4asp_character (Utilities|Casting|CastToUe4ASP_Character OtherActor))
    (Variables|Default|Setoutside false)
    (if (Variables|/Game/AnimStarterPack/Ue4ASP_Character.Ue4ASP_Character_C|GetGasMask _asue_4asp_character) :!label _label
      (Default|GasmaskRealibityDecrease _asue_4asp_character)
      (else
        (Default|RadiationIncrease _asue_4asp_character)))
    (Utilities|FlowControl|Delay 0.2)
    (if (not (Variables|Default|Getoutside))
      (goto _label))))

(event OnComponentEndOverlap(ToxicCol)
  (params (OverlappedComponent :type Primitive%20Component%20Object%20Reference) (OtherActor :type Actor%20Object%20Reference) (OtherComp :type Primitive%20Component%20Object%20Reference) (OtherBodyIndex :type Integer))
  ;[0 1 0] Toxic
  (if (Variables|Default|Gettoxiced)
    (Utilities|Casting|CastToUe4ASP_Character OtherActor)
    (Variables|Default|Setoutside true)))

(event Custom|OpenTheDoor
  (bind _as_metro_save_game (Variables|Default|GetAs%20Metro%20Save%20Game))
  (bind _as_metro_save_game_2 (Variables|Default|GetAs%20Metro%20Save%20Game))
  (bind _tunnellevel (Variables|/Game/GameModes/MetroSaveGame.MetroSaveGame_C|GetTunnelLevel _as_metro_save_game))
  (bind _tunnellevel_2 (Variables|/Game/GameModes/MetroSaveGame.MetroSaveGame_C|GetTunnelLevel _as_metro_save_game_2))
  ;[0 1 0] OpenDoor-CreateNewTunnels
  (Utilities|FlowControl|Sequence
    (:then_0
      (Audio|PlaySoundatLocation "/Game/SFX/NewGateSound.NewGateSound" (Transformation|GetWorldLocation (Variables|Default|GetGateDoor)) "0, 0, 0" 1.0 1.0 0.0 "/Game/SFX/Natural.Natural" 0 0 0)
      (bind _gateopening (Timeline|Timeline_0 Play)
        (:Update
          (Transformation|SetRelativeRotation (Variables|Default|GetGateDoor) (Math|Rotator|MakeRotator 0.0 0.0 (.z _gateopening)) false false))))
    (:then_1
      (Variables|Default|SetNumber (Math|Random|RandomIntegerinRange 0 3) :!label _label)
      (if (== (Variables|Default|GetNumber) 0)
        (Variables|Default|SetMetroClass "/Game/Tunnels/Normal_Tunnel_BP.Normal_Tunnel_BP_C")
        (elif (== (Variables|Default|GetNumber) 1)
          (Variables|Default|SetMetroClass "/Game/Tunnels/Left_Tunnel_BP.Left_Tunnel_BP_C")
          (elif (== (Variables|Default|GetNumber) 2)
            (Variables|Default|SetMetroClass "/Game/Tunnels/Right_Tunnel_BP.Right_Tunnel_BP_C")
            (elif (and (== (Variables|Default|GetNumber) 3) (or (== _tunnellevel_2 0) (== _tunnellevel_2 -1)))
              (Variables|Default|SetMetroClass "/Game/Tunnels/Up_Tunnel_BP.Up_Tunnel_BP_C")
              (elif (and (== (Variables|Default|GetNumber) 3) (or (== _tunnellevel 0) (== _tunnellevel 1)))
                (Variables|Default|SetMetroClass "/Game/Tunnels/Down_Tunnel_BP.Down_Tunnel_BP_C")
                (else
                  (goto _label)))))))
      (Game|SpawnActorfromClass (Variables|Default|GetMetroClass) (Transformation|GetWorldTransform (Variables|Default|GetMetroSpawnPoint)) "Undefined" "SelectDefaultAtRuntime" 0 0)
      (bind _returnvalue (SaveGame|DoesSaveGameExist "metro"))
      (if _returnvalue
        (bind _returnvalue_2 (SaveGame|LoadGamefromSlot "metro"))
        (bind _asmetro_save_game (Utilities|Casting|CastToMetroSaveGame _returnvalue_2))
        (Math|Integer|IncrementInt (Variables|/Game/GameModes/MetroSaveGame.MetroSaveGame_C|GetMetroOpened _asmetro_save_game)
          (:%20%20
            (SaveGame|SaveGametoSlot _asmetro_save_game "metro")))
        (else
          (bind _returnvalue_3 (SaveGame|CreateSaveGameObject "/Game/GameModes/MetroSaveGame.MetroSaveGame_C"))
          (Math|Integer|IncrementInt (Variables|/Game/GameModes/MetroSaveGame.MetroSaveGame_C|GetMetroOpened _returnvalue_3)
            (:%20%20
              (SaveGame|SaveGametoSlot _returnvalue_3 "metro"))))))))

(event Custom|CloseTheDoor
  (bind _gatedoor (Variables|Default|GetGateDoor))
  ;[0 1 0] OpenDoor-CreateNewTunnels
  (Audio|PlaySoundatLocation "/Game/SFX/NewGateSound.NewGateSound" (Transformation|GetWorldLocation _gatedoor) "0, 0, 0" 1.0 1.0 0.0 "/Game/SFX/Natural.Natural" 0 0 0)
  (bind _gateopening (Timeline|Timeline_0 Reverse)
    (:Update
      (Transformation|SetRelativeRotation _gatedoor (Math|Rotator|MakeRotator 0.0 0.0 (.z _gateopening)) false false))))

(event Custom|RandomEvent
  (bind _returnvalue (Math|Random|RandomBool))
  (bind _toxicdeath (Variables|Default|GetToxicDeath))
  (bind _cartplacegood (Variables|Default|GetCartPlaceGood))
  (bind _cartplacebad (Variables|Default|GetCartPlaceBad))
  (bind _toxic (Variables|Default|GetToxic))
  (bind _returnvalue_2 (Transformation|GetWorldTransform _toxic))
  (bind _returnvalue_3 (Transformation|GetWorldTransform _cartplacebad))
  (bind _returnvalue_4 (Transformation|GetWorldTransform _cartplacegood))
  (bind _returnvalue_5 (Transformation|GetWorldTransform _toxicdeath))
  (bind _returnvalue_6 (Math|Transform|SelectTransform _returnvalue_4 _returnvalue_3 _returnvalue))
  (Variables|Default|SetRandomEventInt (Math|Random|RandomIntegerinRange 0 11))
  ;[0 1 0] RandomEvent
  (if (not (Math|Boolean|ORBoolean (== (Variables|Default|GetRandomEventInt) 0) (== (Variables|Default|GetRandomEventInt) 1) (== (Variables|Default|GetRandomEventInt) 2)))
    (if (or (== (Variables|Default|GetRandomEventInt) 3) (== (Variables|Default|GetRandomEventInt) 4))
      (bind _returnvalue_7 (Game|SpawnActorfromClass "/Game/MegascansModels/Imported_Assets/Cart/Cart_BP.Cart_BP_C" (Math|Transform|MakeTransform (Math|Vector|MakeVector (.x (.location _returnvalue_6)) (.y (.location _returnvalue_6)) (.z (.location _returnvalue_6))) (.rotation _returnvalue_6) (.scale _returnvalue_6)) "Undefined" "OverrideRootScale" 0 0))
      (Utilities|Array|Add (Variables|Default|GetSpawnedObject) _returnvalue_7)
      (if (Variables|/Game/MegascansModels/Imported_Assets/Cart/Cart_BP.Cart_BP_C|Getdummy _returnvalue_7)
        (bind _outactors (Actor|GetAllActorsOfClass "/Game/MegascansModels/Imported_Assets/Dummy/Dummy.Dummy_C"))
        (Utilities|Array|Add (Variables|Default|GetSpawnedObject) (Utilities|Array|Get(acopy) _outactors)))
      (elif (or (== (Variables|Default|GetRandomEventInt) 5) (== (Variables|Default|GetRandomEventInt) 6))
        (Game|SpawnActorfromClass "/Game/Ai/Parasite/Parasite_BP.Parasite_BP_C" (Transformation|GetWorldTransform (Variables|Default|GetMutantSpawner1)) "Undefined" "MultiplyWithRoot" 0 0)
        (elif (or (== (Variables|Default|GetRandomEventInt) 7) (== (Variables|Default|GetRandomEventInt) 8))
          (bind _returnvalue_8 (Niagara|SpawnSystematLocation "/Game/VFX/Smoke/SmokeNew_NS.SmokeNew_NS" (.location _returnvalue_2) (.rotation _returnvalue_2) "1.000000,1.000000,1.000000" false))
          (Variables|Default|SetSmokeVar _returnvalue_8)
          (bind _returnvalue_9 (Audio|SpawnSoundatLocation "/Game/SFX/Gas/Gas.Gas" (.location _returnvalue_2) "0, 0, 0" 1.0 1.0 0.0 "/Game/SFX/Atmosphere.Atmosphere" 0))
          (Variables|Default|SetRadiatitonVar _returnvalue_9)
          (Variables|Default|Settoxiced true)
          (if (Math|Random|RandomBool)
            (bind _returnvalue_10 (Game|SpawnActorfromClass "/Game/MegascansModels/Imported_Assets/Dummy/Dummy.Dummy_C" (Math|Transform|MakeTransform (Math|Vector|MakeVector (.x (.location _returnvalue_5)) (.y (.location _returnvalue_5)) (.z (.location _returnvalue_5))) (.rotation _returnvalue_5) (.scale _returnvalue_5)) "Undefined" "OverrideRootScale" 0 0))
            (Utilities|Array|Add (Variables|Default|GetSpawnedObject) _returnvalue_10))
          (elif (== (Variables|Default|GetRandomEventInt) 9)
            (bind _asue_4asp_character (Utilities|Casting|CastToUe4ASP_Character (Game|GetPlayerCharacter 0)))
            (Default|SaveGameSaves _asue_4asp_character)
            (Utilities|FlowControl|Delay 0.3)
            (Game|OpenLevel(byName) "StationLevel")
            (elif (== (Variables|Default|GetRandomEventInt) 10)
              (Game|SpawnActorfromClass "/Game/Ai/Mutant/Mutant_BP.Mutant_BP_C" (Transformation|GetWorldTransform (Variables|Default|GetMutantSpawner1)) "Undefined" "MultiplyWithRoot" 0 0)
              (elif (== (Variables|Default|GetRandomEventInt) 11)
                (Game|SpawnActorfromClass "/Game/Ai/Drake/Drake_BP.Drake_BP_C" (Transformation|GetWorldTransform (Variables|Default|GetMutantSpawner1)) "Undefined" "MultiplyWithRoot" 0 0)))))))))

(event EventBeginPlay
  ;[0 1 0] BeginPlay
  (Utilities|FlowControl|Sequence
    (:then_0
      (bind _returnvalue (SaveGame|DoesSaveGameExist "tunnel"))
      (if _returnvalue
        (bind _returnvalue_2 (SaveGame|LoadGamefromSlot "tunnel"))
        (bind _asmetro_save_game (Utilities|Casting|CastToMetroSaveGame _returnvalue_2))
        (Variables|Default|SetAs%20Metro%20Save%20Game _asmetro_save_game)
        (else
          (bind _returnvalue_3 (SaveGame|CreateSaveGameObject "/Game/GameModes/MetroSaveGame.MetroSaveGame_C"))
          (Variables|Default|SetAs%20Metro%20Save%20Game _returnvalue_3))))
    (:then_1
      (CallFunction|RandomEvent))
    (:then_2
      (if (Math|Random|RandomBool)
        (if (Math|Random|RandomBool)
          (bind _returnvalue_4 (Audio|SpawnSoundatLocation "/Game/SFX/dripping-water-in-cave-114694__mp3cut_net___1_.dripping-water-in-cave-114694__mp3cut_net___1_" (Transformation|GetWorldLocation (Variables|Default|GetTunnel)) "0, 0, 0" 1.0 1.0 0.0 "/Game/SFX/Atmosphere.Atmosphere" 0 false))
          (Variables|Default|SetDrippingSoundVar _returnvalue_4))))))

(fn ConstructionScript)