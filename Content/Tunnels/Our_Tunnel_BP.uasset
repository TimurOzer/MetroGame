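; Tunnel segment for an endless metro that lowers the saved TunnelLevel on BeginPlay and has the player character save.
; The first trigger swings the gate open, spawns a random next tunnel and increments the saved MetroOpened count.
; Up and down tunnels depend on TunnelLevel, rerolling when disallowed.
; Later one-shot triggers close the gate and destroy SpawnedObject actors after a delay, or destroy this segment after a delay.
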(event OnComponentBeginOverlap(Box)
  (params (OverlappedComponent :type Primitive%20Component%20Object%20Reference) (OtherActor :type Actor%20Object%20Reference) (OtherComp :type Primitive%20Component%20Object%20Reference) (OtherBodyIndex :type Integer) (bFromSweep :type Boolean) (SweepResult :type Hit%20Result%20Structure%20%28by%20ref%29))
  ;[0 1 0] OpenDoor-CreateNewTunnels
  (Utilities|Casting|CastToUe4ASP_Character OtherActor)
  (Utilities|FlowControl|DoOnce false
    (:Completed
      (CallFunction|OpentheDoor))))

(event OnComponentBeginOverlap(CloseDoorBox1)
  (params (OverlappedComponent :type Primitive%20Component%20Object%20Reference) (OtherActor :type Actor%20Object%20Reference) (OtherComp :type Primitive%20Component%20Object%20Reference) (OtherBodyIndex :type Integer) (bFromSweep :type Boolean) (SweepResult :type Hit%20Result%20Structure%20%28by%20ref%29))
  ;[0 1 0] DestoryTunnel
  (Utilities|Casting|CastToUe4ASP_Character OtherActor)
  (Utilities|FlowControl|DoOnce false
    (:Completed
      (Utilities|FlowControl|Delay 7.0)
      (Actor|DestroyActor))))

(event OnComponentBeginOverlap(CloseDoorBox)
  (params (OverlappedComponent :type Primitive%20Component%20Object%20Reference) (OtherActor :type Actor%20Object%20Reference) (OtherComp :type Primitive%20Component%20Object%20Reference) (OtherBodyIndex :type Integer) (bFromSweep :type Boolean) (SweepResult :type Hit%20Result%20Structure%20%28by%20ref%29))
  ;[0 1 0] CloseDoor-Destroy
  (Utilities|Casting|CastToUe4ASP_Character OtherActor)
  (Utilities|FlowControl|DoOnce false
    (:Completed
      (CallFunction|ClosetheDoor)
      (Utilities|FlowControl|Delay 5.0)
      (for _array_element (Variables|Default|GetSpawnedObject)
        (Actor|DestroyActor _array_element)))))

(event Custom|OpenTheDoor
  (bind _as_metro_save_game (Variables|Default|GetAs%20Metro%20Save%20Game))
  (bind _as_metro_save_game_2 (Variables|Default|GetAs%20Metro%20Save%20Game))
  (bind _tunnellevel (Variables|/Game/GameModes/MetroSaveGame.MetroSaveGame_C|GetTunnelLevel _as_metro_save_game))
  (bind _tunnellevel_2 (Variables|/Game/GameModes/MetroSaveGame.MetroSaveGame_C|GetTunnelLevel _as_metro_save_game_2))
  ;[0 1 0] OpenDoor-CreateNewTunnels
  (Utilities|FlowControl|Sequence
    (:then_0
      (Audio|PlaySoundatLocation "/Game/SFX/NewGateSound.NewGateSound" (Transformation|GetWorldLocation (Variables|Default|GetGateDoor)) "0, 0, 0" 1.0 1.0 0.0 "/Game/SFX/Natural.Natural" 0 0 0)
      (bind _gateopening (Timeline|Timeline_0 Play)
        (:Update
          (Transformation|SetRelativeRotation (Variables|Default|GetGateDoor) (Math|Rotator|MakeRotator 0.0 0.0 (.z _gateopening)) false false))))
    (:then_1
      (Variables|Default|SetNumber (Math|Random|RandomIntegerinRange 0 3) :!label _label)
      (if (== (Variables|Default|GetNumber) 0)
        (Variables|Default|SetMetroClass "/Game/Tunnels/Normal_Tunnel_BP.Normal_Tunnel_BP_C")
        (elif (== (Variables|Default|GetNumber) 1)
          (Variables|Default|SetMetroClass "/Game/Tunnels/Left_Tunnel_BP.Left_Tunnel_BP_C")
          (elif (== (Variables|Default|GetNumber) 2)
            (Variables|Default|SetMetroClass "/Game/Tunnels/Right_Tunnel_BP.Right_Tunnel_BP_C")
            (elif (and (== (Variables|Default|GetNumber) 3) (or (== _tunnellevel_2 0) (== _tunnellevel_2 -1)))
              (Variables|Default|SetMetroClass "/Game/Tunnels/Up_Tunnel_BP.Up_Tunnel_BP_C")
              (elif (and (== (Variables|Default|GetNumber) 3) (or (== _tunnellevel 0) (== _tunnellevel 1)))
                (Variables|Default|SetMetroClass "/Game/Tunnels/Down_Tunnel_BP.Down_Tunnel_BP_C")
                (else
                  (goto _label)))))))
      (Game|SpawnActorfromClass (Variables|Default|GetMetroClass) (Transformation|GetWorldTransform (Variables|Default|GetMetroSpawnPoint)) "Undefined" "SelectDefaultAtRuntime" 0 0)
      (bind _returnvalue (SaveGame|DoesSaveGameExist "metro"))
      (if _returnvalue
        (bind _returnvalue_2 (SaveGame|LoadGamefromSlot "metro"))
        (bind _asmetro_save_game (Utilities|Casting|CastToMetroSaveGame _returnvalue_2))
        (Math|Integer|IncrementInt (Variables|/Game/GameModes/MetroSaveGame.MetroSaveGame_C|GetMetroOpened _asmetro_save_game)
          (:%20%20
            (SaveGame|SaveGametoSlot _asmetro_save_game "metro")))
        (else
          (bind _returnvalue_3 (SaveGame|CreateSaveGameObject "/Game/GameModes/MetroSaveGame.MetroSaveGame_C"))
          (Math|Integer|IncrementInt (Variables|/Game/GameModes/MetroSaveGame.MetroSaveGame_C|GetMetroOpened _returnvalue_3)
            (:%20%20
              (SaveGame|SaveGametoSlot _returnvalue_3 "metro"))))))))

(event Custom|CloseTheDoor
  (bind _gatedoor (Variables|Default|GetGateDoor))
  ;[0 1 0] OpenDoor-CreateNewTunnels
  (Audio|PlaySoundatLocation "/Game/SFX/NewGateSound.NewGateSound" (Transformation|GetWorldLocation _gatedoor) "0, 0, 0" 1.0 1.0 0.0 "/Game/SFX/Natural.Natural" 0 0 0)
  (bind _gateopening (Timeline|Timeline_0 Reverse)
    (:Update
      (Transformation|SetRelativeRotation _gatedoor (Math|Rotator|MakeRotator 0.0 0.0 (.z _gateopening)) false false))))

(event Custom|RandomEvent
  ;[0 1 0] RandomEvent
  (if (not (Math|Random|RandomBool))
    (if (not (Math|Random|RandomBool))
      (if (Math|Random|RandomBool)
        _))))

(event EventBeginPlay
  ;[0 1 0] BeginPlay
  (Utilities|FlowControl|Sequence
    (:then_0
      (bind _returnvalue (SaveGame|DoesSaveGameExist "tunnel"))
      (if _returnvalue
        (bind _returnvalue_2 (SaveGame|LoadGamefromSlot "tunnel"))
        (bind _asmetro_save_game (Utilities|Casting|CastToMetroSaveGame _returnvalue_2))
        (Math|Integer|DecrementInt (Variables|/Game/GameModes/MetroSaveGame.MetroSaveGame_C|GetTunnelLevel _asmetro_save_game)
          (:%20%20
            (SaveGame|SaveGametoSlot _asmetro_save_game "tunnel")))
        (else
          (bind _returnvalue_3 (SaveGame|CreateSaveGameObject "/Game/GameModes/MetroSaveGame.MetroSaveGame_C"))
          (Math|Integer|DecrementInt (Variables|/Game/GameModes/MetroSaveGame.MetroSaveGame_C|GetTunnelLevel _returnvalue_3)
            (:%20%20
              (SaveGame|SaveGametoSlot _returnvalue_3 "tunnel"))))))
    (:then_1
      (bind _asue_4asp_character (Utilities|Casting|CastToUe4ASP_Character (Game|GetPlayerCharacter 0)))
      (Default|SaveGameSaves _asue_4asp_character))))

(fn ConstructionScript)