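; Up tunnel segment of a randomly chained metro, with gate and tunnel count saved.
; BeginPlay randomizes rubble, dripping audio and one possible event: toxic gas, creature, cart or save-and-jump to StationLevel.
; Player overlaps open the gate, spawning another tunnel type or loading the station, then later close it, clean up props and destroy the segment.
; Toxic gas loops on a delay, wearing down the gas mask or raising radiation.
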(event OnComponentBeginOverlap(Box)
  (params (OverlappedComponent :type Primitive%20Component%20Object%20Reference) (OtherActor :type Actor%20Object%20Reference) (OtherComp :type Primitive%20Component%20Object%20Reference) (OtherBodyIndex :type Integer) (bFromSweep :type Boolean) (SweepResult :type Hit%20Result%20Structure%20%28by%20ref%29))
  ;[0 1 0] OpenDoor-CreateNewTunnels
  (Utilities|Casting|CastToUe4ASP_Character OtherActor)
  (Utilities|FlowControl|DoOnce false
    (:Completed
      (CallFunction|OpentheDoor))))

(event OnComponentBeginOverlap(CloseDoorBox1)
  (params (OverlappedComponent :type Primitive%20Component%20Object%20Reference) (OtherActor :type Actor%20Object%20Reference) (OtherComp :type Primitive%20Component%20Object%20Reference) (OtherBodyIndex :type Integer) (bFromSweep :type Boolean) (SweepResult :type Hit%20Result%20Structure%20%28by%20ref%29))
  ;[0 1 0] DestoryTunnel
  (Utilities|Casting|CastToUe4ASP_Character OtherActor)
  (Utilities|FlowControl|DoOnce false
    (:Completed
      (Utilities|FlowControl|Delay 7.0)
      (Actor|DestroyActor))))

(event OnComponentBeginOverlap(CloseDoorBox)
  (params (OverlappedComponent :type Primitive%20Component%20Object%20Reference) (OtherActor :type Actor%20Object%20Reference) (OtherComp :type Primitive%20Component%20Object%20Reference) (OtherBodyIndex :type Integer) (bFromSweep :type Boolean) (SweepResult :type Hit%20Result%20Structure%20%28by%20ref%29))
  (bind _smokevar (Variables|Default|GetSmokeVar))
  (bind _radiatitonvar (Variables|Default|GetRadiatitonVar))
  (bind _drippingsoundvar (Variables|Default|GetDrippingSoundVar))
  ;[0 1 0] CloseDoor-Destroy
  (Utilities|Casting|CastToUe4ASP_Character OtherActor)
  (Utilities|FlowControl|DoOnce false
    (:Completed
      (CallFunction|ClosetheDoor)
      (Utilities|FlowControl|Delay 5.0)
      (Utilities|IsValid _drippingsoundvar
        (:Is%20Valid
          (Components|DestroyComponent _drippingsoundvar))
        (:Is%20Not%20Valid
          _))
      (Utilities|IsValid _smokevar
        (:Is%20Valid
          (Components|DestroyComponent _smokevar))
        (:Is%20Not%20Valid
          _))
      (Utilities|IsValid _radiatitonvar
        (:Is%20Valid
          (Components|DestroyComponent _radiatitonvar))
        (:Is%20Not%20Valid
          _))
      (for _array_element (Variables|Default|GetSpawnedObject)
        (Actor|DestroyActor _array_element)))))

(event OnComponentBeginOverlap(ToxicCol)
  (params (OverlappedComponent :type Primitive%20Component%20Object%20Reference) (OtherActor :type Actor%20Object%20Reference) (OtherComp :type Primitive%20Component%20Object%20Reference) (OtherBodyIndex :type Integer) (bFromSweep :type Boolean) (SweepResult :type Hit%20Result%20Structure%20%28by%20ref%29))
  ;[0 1 0] Toxic
  (if (Variables|Default|Gettoxiced)
    (bind _asue_4asp_character (Utilities|Casting|CastToUe4ASP_Character OtherActor))
    (Variables|Default|Setoutside false)
    (if (Variables|/Game/AnimStarterPack/Ue4ASP_Character.Ue4ASP_Character_C|GetGasMask _asue_4asp_character) :!label _label
      (Default|GasmaskRealibityDecrease _asue_4asp_character)
      (else
        (Default|RadiationIncrease _asue_4asp_character)))
    (Utilities|FlowControl|Delay 0.2)
    (if (not (Variables|Default|Getoutside))
      (goto _label))))

(event OnComponentEndOverlap(ToxicCol)
  (params (OverlappedComponent :type Primitive%20Component%20Object%20Reference) (OtherActor :type Actor%20Object%20Reference) (OtherComp :type Primitive%20Component%20Object%20Reference) (OtherBodyIndex :type Integer))
  ;[0 1 0] Toxic
  (if (Variables|Default|Gettoxiced)
    (Utilities|Casting|CastToUe4ASP_Character OtherActor)
    (Variables|Default|Setoutside true)))

(event Custom|OpenTheDoor
  ;[0 1 0] OpenDoor-CreateNewTunnels
  (Utilities|FlowControl|Sequence
    (:then_0
      (Audio|PlaySoundatLocation "/Game/SFX/NewGateSound.NewGateSound" (Transformation|GetWorldLocation (Variables|Default|GetGateDoor)) "0, 0, 0" 1.0 1.0 0.0 "/Game/SFX/Natural.Natural" 0 0 0)
      (bind _gateopening (Timeline|Timeline_0 Play)
        (:Update
          (Transformation|SetRelativeRotation (Variables|Default|GetGateDoor) (Math|Rotator|MakeRotator 0.0 0.0 (.z _gateopening)) false false))))
    (:then_1
      (if (== (Math|Random|RandomIntegerinRange 0 9) 9)
        (bind _asue_4asp_character (Utilities|Casting|CastToUe4ASP_Character (Game|GetPlayerCharacter 0)))
        (Default|SaveGameSaves _asue_4asp_character)
        (Game|OpenLevel(byName) "StationLevel")
        (else
          (Variables|Default|SetNumber (Math|Random|RandomIntegerinRange 0 3))
          (if (== (Variables|Default|GetNumber) 0)
            (Variables|Default|SetMetroClass "/Game/Tunnels/Normal_Tunnel_BP.Normal_Tunnel_BP_C")
            (Game|SpawnActorfromClass (Variables|Default|GetMetroClass) (Transformation|GetWorldTransform (Variables|Default|GetMetroSpawnPoint)) "Undefined" "SelectDefaultAtRuntime" 0 0 :!label _label)
            (bind _returnvalue (SaveGame|DoesSaveGameExist "metro"))
            (if _returnvalue
              (bind _returnvalue_2 (SaveGame|LoadGamefromSlot "metro"))
              (bind _asmetro_save_game (Utilities|Casting|CastToMetroSaveGame _returnvalue_2))
              (Math|Integer|IncrementInt (Variables|/Game/GameModes/MetroSaveGame.MetroSaveGame_C|GetMetroOpened _asmetro_save_game)
                (:%20%20
                  (SaveGame|SaveGametoSlot _asmetro_save_game "metro")))
              (else
                (bind _returnvalue_3 (SaveGame|CreateSaveGameObject "/Game/GameModes/MetroSaveGame.MetroSaveGame_C"))
                (Math|Integer|IncrementInt (Variables|/Game/GameModes/MetroSaveGame.MetroSaveGame_C|GetMetroOpened _returnvalue_3)
                  (:%20%20
                    (SaveGame|SaveGametoSlot _returnvalue_3 "metro")))))
            (elif (== (Variables|Default|GetNumber) 1)
              (Variables|Default|SetMetroClass "/Game/Tunnels/Left_Tunnel_BP.Left_Tunnel_BP_C")
              (goto _label)
              (elif (== (Variables|Default|GetNumber) 2)
                (Variables|Default|SetMetroClass "/Game/Tunnels/Right_Tunnel_BP.Right_Tunnel_BP_C")
                (goto _label)
                (elif (== (Variables|Default|GetNumber) 3)
                  (Variables|Default|SetMetroClass "/Game/Tunnels/Down_Tunnel_BP.Down_Tunnel_BP_C")
                  (goto _label))))))))))

(event Custom|CloseTheDoor
  (bind _gatedoor (Variables|Default|GetGateDoor))
  ;[0 1 0] OpenDoor-CreateNewTunnels
  (Audio|PlaySoundatLocation "/Game/SFX/NewGateSound.NewGateSound" (Transformation|GetWorldLocation _gatedoor) "0, 0, 0" 1.0 1.0 0.0 "/Game/SFX/Natural.Natural" 0 0 0)
  (bind _gateopening (Timeline|Timeline_0 Reverse)
    (:Update
      (Transformation|SetRelativeRotation _gatedoor (Math|Rotator|MakeRotator 0.0 0.0 (.z _gateopening)) false false))))

(event Custom|RandomEvent
  (bind _returnvalue (Math|Random|RandomBool))
  (bind _toxicdeath (Variables|Default|GetToxicDeath))
  (bind _cartplacegood (Variables|Default|GetCartPlaceGood))
  (bind _cartplacebad (Variables|Default|GetCartPlaceBad))
  (bind _toxic (Variables|Default|GetToxic))
  (bind _returnvalue_2 (Transformation|GetWorldTransform _toxic))
  (bind _returnvalue_3 (Transformation|GetWorldTransform _cartplacebad))
  (bind _returnvalue_4 (Transformation|GetWorldTransform _cartplacegood))
  (bind _returnvalue_5 (Transformation|GetWorldTransform _toxicdeath))
  (bind _returnvalue_6 (Math|Transform|SelectTransform _returnvalue_4 _returnvalue_3 _returnvalue))
  ;[0 1 0] RandomEvent
  (if (not (Math|Random|RandomBool))
    (if (Math|Random|RandomBool)
      (bind _returnvalue_7 (Niagara|SpawnSystematLocation "/Game/VFX/Smoke/SmokeNew_NS.SmokeNew_NS" (.location _returnvalue_2) (.rotation _returnvalue_2) "1.000000,1.000000,1.000000" false))
      (Variables|Default|SetSmokeVar _returnvalue_7)
      (bind _returnvalue_8 (Audio|SpawnSoundatLocation "/Game/SFX/Gas/Gas.Gas" (.location _returnvalue_2) "0, 0, 0" 1.0 1.0 0.0 "/Game/SFX/Atmosphere.Atmosphere" 0))
      (Variables|Default|SetRadiatitonVar _returnvalue_8)
      (Variables|Default|Settoxiced true)
      (if (Math|Random|RandomBool)
        (bind _returnvalue_9 (Game|SpawnActorfromClass "/Game/MegascansModels/Imported_Assets/Dummy/Dummy.Dummy_C" (Math|Transform|MakeTransform (Math|Vector|MakeVector (.x (.location _returnvalue_5)) (.y (.location _returnvalue_5)) (.z (.location _returnvalue_5))) (.rotation _returnvalue_5) (.scale _returnvalue_5)) "Undefined" "OverrideRootScale" 0 0))
        (Utilities|Array|Add (Variables|Default|GetSpawnedObject) _returnvalue_9))
      (elif (Math|Random|RandomBool)
        (Game|SpawnActorfromClass "/Game/Ai/Parasite/Parasite_BP.Parasite_BP_C" (Transformation|GetWorldTransform (Variables|Default|GetMutantSpawner1)) "Undefined" "MultiplyWithRoot" 0 0)
        (elif (Math|Random|RandomBool)
          (bind _returnvalue_10 (Game|SpawnActorfromClass "/Game/MegascansModels/Imported_Assets/Cart/Cart_BP.Cart_BP_C" (Math|Transform|MakeTransform (Math|Vector|MakeVector (.x (.location _returnvalue_6)) (.y (.location _returnvalue_6)) (.z (.location _returnvalue_6))) (.rotation _returnvalue_6) (.scale _returnvalue_6)) "Undefined" "OverrideRootScale" 0 0))
          (Utilities|Array|Add (Variables|Default|GetSpawnedObject) _returnvalue_10)
          (if (Variables|/Game/MegascansModels/Imported_Assets/Cart/Cart_BP.Cart_BP_C|Getdummy _returnvalue_10)
            (bind _outactors (Actor|GetAllActorsOfClass "/Game/MegascansModels/Imported_Assets/Dummy/Dummy.Dummy_C"))
            (Utilities|Array|Add (Variables|Default|GetSpawnedObject) (Utilities|Array|Get(acopy) _outactors)))
          (elif (Math|Random|RandomBool)
            (bind _asue_4asp_character (Utilities|Casting|CastToUe4ASP_Character (Game|GetPlayerCharacter 0)))
            (Default|SaveGameSaves _asue_4asp_character)
            (Game|OpenLevel(byName) "StationLevel")
            (elif (Math|Random|RandomBool)
              (Game|SpawnActorfromClass "/Game/Ai/Mutant/Mutant_BP.Mutant_BP_C" (Transformation|GetWorldTransform (Variables|Default|GetMutantSpawner1)) "Undefined" "MultiplyWithRoot" 0 0)
              (elif (Math|Random|RandomBool)
                (Game|SpawnActorfromClass "/Game/Ai/Drake/Drake_BP.Drake_BP_C" (Transformation|GetWorldTransform (Variables|Default|GetMutantSpawner1)) "Undefined" "MultiplyWithRoot" 0 0)))))))))

(event EventBeginPlay
  ;[0 1 0] BeginPlay
  (Utilities|FlowControl|Sequence
    (:then_0
      (bind _returnvalue (SaveGame|DoesSaveGameExist "tunnel"))
      (if _returnvalue
        (bind _returnvalue_2 (SaveGame|LoadGamefromSlot "tunnel"))
        (bind _asmetro_save_game (Utilities|Casting|CastToMetroSaveGame _returnvalue_2))
        (Math|Integer|IncrementInt (Variables|/Game/GameModes/MetroSaveGame.MetroSaveGame_C|GetTunnelLevel _asmetro_save_game)
          (:%20%20
            (SaveGame|SaveGametoSlot _asmetro_save_game "tunnel")))
        (else
          (bind _returnvalue_3 (SaveGame|CreateSaveGameObject "/Game/GameModes/MetroSaveGame.MetroSaveGame_C"))
          (Math|Integer|IncrementInt (Variables|/Game/GameModes/MetroSaveGame.MetroSaveGame_C|GetTunnelLevel _returnvalue_3)
            (:%20%20
              (SaveGame|SaveGametoSlot _returnvalue_3 "tunnel"))))))
    (:then_1
      (CallFunction|RandomEvent)
      (Utilities|FlowControl|Sequence
        (:then_0
          (Utilities|FlowControl|Sequence))
        (:then_1
          (if (Math|Random|RandomBool)
            (Components|DestroyComponent (Variables|Default|GetS_Cement_Rubble_rkCty_lod21))))
        (:then_2
          (if (Math|Random|RandomBool)
            (Components|DestroyComponent (Variables|Default|GetS_Cement_Rubble_rkCty_lod19))))
        (:then_3
          (if (Math|Random|RandomBool)
            (Components|DestroyComponent (Variables|Default|GetS_Cement_Rubble_rkCty_lod18))))
        (:then_4
          (if (Math|Random|RandomBool)
            (Components|DestroyComponent (Variables|Default|GetS_Cement_Rubble_rkCty_lod17))))
        (:then_5
          (if (Math|Random|RandomBool)
            (Components|DestroyComponent (Variables|Default|GetS_Cement_Rubble_rkCty_lod20))))
        (:then_6
          (if (Math|Random|RandomBool)
            (Components|DestroyComponent (Variables|Default|GetS_Cement_Rubble_rkCty_lod16))))
        (:then_7
          (if (Math|Random|RandomBool)
            (Components|DestroyComponent (Variables|Default|GetS_Cement_Rubble_rkCty_lod15))))
        (:then_8
          (if (Math|Random|RandomBool)
            (Components|DestroyComponent (Variables|Default|GetS_Cement_Rubble_rkCty_lod14))))
        (:then_9
          (if (Math|Random|RandomBool)
            (Components|DestroyComponent (Variables|Default|GetS_Cement_Rubble_rkCty_lod27))))
        (:then_10
          (if (Math|Random|RandomBool)
            (Components|DestroyComponent (Variables|Default|GetS_Cement_Rubble_rkCty_lod26))))
        (:then_11
          (if (Math|Random|RandomBool)
            (Components|DestroyComponent (Variables|Default|GetS_Cement_Rubble_rkCty_lod25))))
        (:then_12
          (if (Math|Random|RandomBool)
            (Components|DestroyComponent (Variables|Default|GetS_Cement_Rubble_rkCty_lod6))))
        (:then_13
          (if (Math|Random|RandomBool)
            (Components|DestroyComponent (Variables|Default|GetS_Cement_Rubble_rkCty_lod24))))
        (:then_14
          (if (Math|Random|RandomBool)
            (Components|DestroyComponent (Variables|Default|GetS_Cement_Rubble_rkCty_lod23))))
        (:then_15
          (if (Math|Random|RandomBool)
            (Components|DestroyComponent (Variables|Default|GetS_Cement_Rubble_rkCty_lod22))))
        (:then_16
          (if (Math|Random|RandomBool)
            (Components|DestroyComponent (Variables|Default|GetS_Cement_Rubble_rkCty_lod13))))
        (:then_17
          (if (Math|Random|RandomBool)
            (Components|DestroyComponent (Variables|Default|GetS_Cement_Rubble_rkCty_lod12))))
        (:then_18
          (if (Math|Random|RandomBool)
            (Components|DestroyComponent (Variables|Default|GetS_Cement_Rubble_rkCty_lod11))))
        (:then_19
          (if (Math|Random|RandomBool)
            (Components|DestroyComponent (Variables|Default|GetS_Cement_Rubble_rkCty_lod10))))
        (:then_20
          (if (Math|Random|RandomBool)
            (Components|DestroyComponent (Variables|Default|GetS_Cement_Rubble_rkCty_lod9))))
        (:then_21
          (if (Math|Random|RandomBool)
            (Components|DestroyComponent (Variables|Default|GetS_Cement_Rubble_rkCty_lod5))))
        (:then_22
          (if (Math|Random|RandomBool)
            (Components|DestroyComponent (Variables|Default|GetS_Cement_Rubble_rkCty_lod8))))
        (:then_23
          (if (Math|Random|RandomBool)
            (Components|DestroyComponent (Variables|Default|GetS_Cement_Rubble_rkCty_lod7))))))
    (:then_2
      (if (Math|Random|RandomBool)
        (bind _returnvalue_4 (Audio|SpawnSoundatLocation "/Game/SFX/dripping-water-in-cave-114694__mp3cut_net___1_.dripping-water-in-cave-114694__mp3cut_net___1_" (Transformation|GetWorldLocation (Variables|Default|GetTunnel)) "0, 0, 0" 1.0 1.0 0.0 "/Game/SFX/Atmosphere.Atmosphere" 0 false))
        (Variables|Default|SetDrippingSoundVar _returnvalue_4)))))

(fn ConstructionScript)