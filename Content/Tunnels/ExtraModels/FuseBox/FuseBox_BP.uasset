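; Interactable tunnel fuse box that switches on the lights of its tunnel through TunnelCreator's OpenLight.
; Interacting records TunnelName in the LightOpened map of a KharkivSaveGame in the "lighttunnel" slot, then sets the box meshes to physics-only collision.
; BeginPlay reads that map and reapplies only the collision change for tunnels already lit.
; The construction script randomly shows one of two box-and-voltmeter mesh pairs.
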(event EventBeginPlay
  (bind _returnvalue (SaveGame|DoesSaveGameExist "lighttunnel"))
  (if _returnvalue
    (bind _returnvalue_2 (SaveGame|LoadGamefromSlot "lighttunnel"))
    (bind _askharkiv_save_game (Utilities|Casting|CastToKharkivSaveGame _returnvalue_2))
    (if (.Value (Utilities|Map|Find (Variables|/Game/GameModes/KharkivSaveGame.KharkivSaveGame_C|GetLightOpened _askharkiv_save_game) (Variables|Default|GetTunnelName)))
      (Collision|SetCollisionEnabled (Variables|Default|Getuploads_files_3146259_Electricalbox_Voltmeter) "PhysicsOnly" :!label _label))
    (else
      (bind _returnvalue_3 (SaveGame|CreateSaveGameObject "/Game/GameModes/KharkivSaveGame.KharkivSaveGame_C"))
      (if (.Value (Utilities|Map|Find (Variables|/Game/GameModes/KharkivSaveGame.KharkivSaveGame_C|GetLightOpened _returnvalue_3) (Variables|Default|GetTunnelName)))
        (goto _label)))))

(event EventInteractingObject
  (bind _returnvalue (SaveGame|DoesSaveGameExist "lighttunnel"))
  (if _returnvalue
    (bind _returnvalue_2 (SaveGame|LoadGamefromSlot "lighttunnel"))
    (bind _askharkiv_save_game (Utilities|Casting|CastToKharkivSaveGame _returnvalue_2))
    (Utilities|Map|Add (Variables|/Game/GameModes/KharkivSaveGame.KharkivSaveGame_C|GetLightOpened _askharkiv_save_game) (Variables|Default|GetTunnelName) true)
    (SaveGame|SaveGametoSlot _askharkiv_save_game "lighttunnel")
    (else
      (bind _returnvalue_3 (SaveGame|CreateSaveGameObject "/Game/GameModes/KharkivSaveGame.KharkivSaveGame_C"))
      (Utilities|Map|Add (Variables|/Game/GameModes/KharkivSaveGame.KharkivSaveGame_C|GetLightOpened _returnvalue_3) (Variables|Default|GetTunnelName) true)
      (SaveGame|SaveGametoSlot _returnvalue_3 "lighttunnel")))
  (Collision|SetCollisionEnabled (Variables|Default|Getuploads_files_3146259_Electricalbox_Voltmeter) "PhysicsOnly")
  (Default|OpenLight (Variables|Default|GetTunnelCreator)))

(fn ConstructionScript
  (if (Math|Random|RandomBool)
    (Rendering|SetVisibility (Variables|Default|Getuploads_files_3146259_Electricalbox_Voltmeter) true false)
    (else
      (Rendering|SetVisibility (Variables|Default|Getuploads_files_3146259_Electricalbox_Voltmeter001) true false))))