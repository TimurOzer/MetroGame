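; Grafiti_BP is a tunnel decal actor that places randomized graffiti.
; The Construction Script creates a dynamic material instance on the decal and sets its texture parameter to one of thirty textures picked at random.
; It also randomizes the material's rotation parameter and the decal's width and height, keeping the depth thin.
; All variation happens at construction with unseeded random nodes, and the event graph is empty.
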(event EventBeginPlay)

(event Collision|EventActorBeginOverlap
  (params (OtherActor :type Actor%20Object%20Reference)))

(event EventTick
  (params (DeltaSeconds :type Float%20%28single-precision%29)))

(fn ConstructionScript
  (bind _returnvalue (Rendering|Material|CreateDynamicMaterialInstance (Variables|Default|GetDecal) :!class /Script/Engine.DecalComponent))
  (Rendering|Material|SetTextureParameterValue _returnvalue "Texture" (Utilities|Select :Index (Math|Random|RandomIntegerinRange 0 29) :Option%200 "/Game/Tunnels/ExtraModels/Grafitties/2RxctC72TlL0.2RxctC72TlL0" :Option%201 "/Game/Tunnels/ExtraModels/Grafitties/3erSGv2mptPb.3erSGv2mptPb" :Option%202 "/Game/Tunnels/ExtraModels/Grafitties/6w1476ONzVZW.6w1476ONzVZW" :Option%203 "/Game/Tunnels/ExtraModels/Grafitties/8I0rLvfVrv2V.8I0rLvfVrv2V" :Option%204 "/Game/Tunnels/ExtraModels/Grafitties/9UXErsmP4cNK.9UXErsmP4cNK" :Option%205 "/Game/Tunnels/ExtraModels/Grafitties/BnWcrmxeYdmM.BnWcrmxeYdmM" :Option%206 "/Game/Tunnels/ExtraModels/Grafitties/Bwz51lKo7XeM.Bwz51lKo7XeM" :Option%207 "/Game/Tunnels/ExtraModels/Grafitties/cCQFqhCat3tF.cCQFqhCat3tF" :Option%208 "/Game/Tunnels/ExtraModels/Grafitties/Dd45tHHW3ZPB.Dd45tHHW3ZPB" :Option%209 "/Game/Tunnels/ExtraModels/Grafitties/dk7QVTC1Nb5a.dk7QVTC1Nb5a" :Option%2010 "/Game/Tunnels/ExtraModels/Grafitties/e7Eadet1wxB4.e7Eadet1wxB4" :Option%2011 "/Game/Tunnels/ExtraModels/Grafitties/ERsze2eaXPDF.ERsze2eaXPDF" :Option%2012 "/Game/Tunnels/ExtraModels/Grafitties/fFSy6deYlrsp.fFSy6deYlrsp" :Option%2013 "/Game/Tunnels/ExtraModels/Grafitties/Fs53Hwh7jIr4.Fs53Hwh7jIr4" :Option%2014 "/Game/Tunnels/ExtraModels/Grafitties/fZp1uE83gCza.fZp1uE83gCza" :Option%2015 "/Game/Tunnels/ExtraModels/Grafitties/G07j5ZtcCwkH.G07j5ZtcCwkH" :Option%2016 "/Game/Tunnels/ExtraModels/Grafitties/jC9ycu4KzFWG.jC9ycu4KzFWG" :Option%2017 "/Game/Tunnels/ExtraModels/Grafitties/JwVNAiIqT8kv.JwVNAiIqT8kv" :Option%2018 "/Game/Tunnels/ExtraModels/Grafitties/reR4ef0beXJi.reR4ef0beXJi" :Option%2019 "/Game/Tunnels/ExtraModels/Grafitties/tbV5HDN0kekJ.tbV5HDN0kekJ" :Option%2020 "/Game/Tunnels/ExtraModels/Grafitties/tW6bSq2Crqfv.tW6bSq2Crqfv" :Option%2021 "/Game/Tunnels/ExtraModels/Grafitties/uEV4TzluAjUj.uEV4TzluAjUj" :Option%2022 "/Game/Tunnels/ExtraModels/Grafitties/UeYw52TocHCt.UeYw52TocHCt" :Option%2023 "/Game/Tunnels/ExtraModels/Grafitties/WNtKe2dChz6A.WNtKe2dChz6A" :Option%2024 "/Game/Tunnels/ExtraModels/Grafitties/X1xd0VNWzroS.X1xd0VNWzroS" :Option%2025 "/Game/Tunnels/ExtraModels/Grafitties/xcprNBxURTCF.xcprNBxURTCF" :Option%2026 "/Game/Tunnels/ExtraModels/Grafitties/xjdQet6eYv5E.xjdQet6eYv5E" :Option%2027 "/Game/Tunnels/ExtraModels/Grafitties/xtvQxwed49mB.xtvQxwed49mB" :Option%2028 "/Game/Tunnels/ExtraModels/Grafitties/yMwNW4OErNoM.yMwNW4OErNoM" :Option%2029 "/Game/Tunnels/ExtraModels/Grafitties/zzDRrLtZIDl9.zzDRrLtZIDl9"))
  (Rendering|Material|SetScalarParameterValue _returnvalue "Rotation" (Math|Random|RandomFloatinRange 0.0 3.6e+02) :!class /Script/Engine.MaterialInstanceDynamic)
  (Transformation|SetWorldScale3D (Variables|Default|GetDecal) (Math|Vector|MakeVector 0.01 (Math|Random|RandomFloatinRange 0.1 0.3) (Math|Random|RandomFloatinRange 0.1 0.3))))